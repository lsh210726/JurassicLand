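; Playable blue T-Rex battle character with bite, roar, a selectable special (flame, laser or ice) and a timed power, defence or speed buff.
; Attacks and buffs go through Server-to-Multicast event pairs, with montages, notifies, traces and spawned projectiles driving effects and damage.
; AnyDamage branches on damage type, using invulnerability windows, an ice slow and hit/death reactions.
; MultiCustom attaches hat, glasses and shoe actors from a data table to body sockets.
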(event `SpawnShoesItemR`
  (bind _trexbody (`self.TRexBody`))
  (bind (_returnvalue_location _returnvalue_rotation) (`KismetMathLibrary.BreakTransform` (`SceneComponent.GetSocketTransform` _trexbody "RightBallSocket" "RTS_World")))
  ;[1 1 1] CUstom Multi  JE
  (bind _returnvalue (`|SpawnActorFromClass` (`self.RShoesActorClass`) (`KismetMathLibrary.MakeTransform` _returnvalue_location _returnvalue_rotation) "Undefined" "MultiplyWithRoot" null null))
  (`self.K2_AttachToComponent` _returnvalue _trexbody "RightBallSocket" "KeepWorld" "KeepWorld" "KeepWorld" true))

(event `SpawnHatItem`
  (bind _trexbody (`self.TRexBody`))
  (bind (_returnvalue_location _returnvalue_rotation) (`KismetMathLibrary.BreakTransform` (`SceneComponent.GetSocketTransform` _trexbody "HeadSocket" "RTS_World")))
  ;[1 1 1] CUstom Multi  JE
  (bind _returnvalue (`|SpawnActorFromClass` (`self.HatActorClass`) (`KismetMathLibrary.MakeTransform` _returnvalue_location _returnvalue_rotation) "Undefined" "MultiplyWithRoot" null null))
  (`self.K2_AttachToComponent` _returnvalue _trexbody "HeadSocket" "KeepWorld" "KeepWorld" "KeepWorld" true))

(event `SpawnGlassesItem`
  (bind _trexbody (`self.TRexBody`))
  (bind (_returnvalue_location _returnvalue_rotation _returnvalue_scale) (`KismetMathLibrary.BreakTransform` (`SceneComponent.GetSocketTransform` _trexbody "RightEyeSocket" "RTS_World")))
  ;[1 1 1] CUstom Multi  JE
  (bind _returnvalue (`|SpawnActorFromClass` (`self.GlassesActorClass`) (`KismetMathLibrary.MakeTransform` _returnvalue_location _returnvalue_rotation _returnvalue_scale) "Undefined" "MultiplyWithRoot" null null))
  (`self.K2_AttachToComponent` _returnvalue _trexbody "RightEyeSocket" "KeepWorld" "KeepWorld" "KeepWorld" true))

(event `SpawnShoesItemL`
  (bind _trexbody (`self.TRexBody`))
  (bind (_returnvalue_location _returnvalue_rotation) (`KismetMathLibrary.BreakTransform` (`SceneComponent.GetSocketTransform` _trexbody "LeftBallSocket" "RTS_World")))
  ;[1 1 1] CUstom Multi  JE
  (bind _returnvalue (`|SpawnActorFromClass` (`self.LShoesActorClass`) (`KismetMathLibrary.MakeTransform` _returnvalue_location _returnvalue_rotation) "Undefined" "MultiplyWithRoot" null null))
  (`self.K2_AttachToComponent` _returnvalue _trexbody "LeftBallSocket" "KeepWorld" "KeepWorld" "KeepWorld" true))

(event `self.InitialCustomMulti`
  ;[1 1 1] CUstom Multi  JE
  (`self.MultiCustom`))

(event `MultiCustom`
  (bind _returnvalue (`KismetTextLibrary.Conv_NameToText` (`self.playerHat`)))
  ;[1 1 1] CUstom Multi  JE
  (cast `/Game/LSH_WorkSpace/BP_LSH_NetGameInstance` (`GameplayStatics.GetGameInstance`))
  (bind _outrownames (`DataTableFunctionLibrary.GetDataTableRowNames` "/Game/7_MISC/ItemData/CustomItemData3.CustomItemData3"))
  (for _array_element _outrownames
    (bind _returnvalue_2 (`|GetDataTableRow` "/Game/7_MISC/ItemData/CustomItemData3.CustomItemData3" _array_element)
      (:`then`
        (bind (_itemtype _itemtextdata _itemassetsdata) (break `JE_CustomItem` _returnvalue_2))
        (if (`|EnumEquality` _itemtype "Hat")
          (if (`KismetTextLibrary.EqualEqual_TextText` (break `ItemTextData` _itemtextdata) _returnvalue)
            (`KismetSystemLibrary.PrintString` (`KismetTextLibrary.Conv_TextToString` _returnvalue) true true (struct :`G` 0.66 :`B` 1.0 :`A` 1.0) (`self.textTime`))
            (bind _output_get (set `self.HatActorClass` (`.ActorMesh` (break `ItemAssetData` _itemassetsdata))))
            (`self.SpawnHatItem`))
          (elif (`|EnumEquality` _itemtype "Glasses")
            (if (`KismetTextLibrary.EqualEqual_TextText` (break `ItemTextData` _itemtextdata) (`KismetTextLibrary.Conv_NameToText` (`self.playerGlasses`)))
              (set `self.GlassesActorClass` (`.ActorMesh` (break `ItemAssetData` _itemassetsdata)))
              (`self.SpawnGlassesItem`))
            (elif (`|EnumEquality` _itemtype "Shoes")
              (if (`KismetTextLibrary.EqualEqual_TextText` (break `ItemTextData` _itemtextdata) (`KismetTextLibrary.Conv_NameToText` (`self.playerShoes`)))
                (if (`KismetTextLibrary.EqualEqual_TextText` (`.Description` (break `ItemTextData` _itemtextdata)) (`KismetTextLibrary.Conv_NameToText` "right"))
                  (set `self.RShoesActorClass` (`.ActorMesh` (break `ItemAssetData` _itemassetsdata)))
                  (`self.SpawnShoesItemR`)
                  (else
                    (set `self.LShoesActorClass` (`.ActorMesh` (break `ItemAssetData` _itemassetsdata)))
                    (`self.SpawnShoesItemL`)))))))))))

(event `self.ReceiveTick`
  (params (DeltaSeconds :type "Float (single-precision)")))

(event `self.ReceiveBeginPlay`
  ;[0.07669 0.9741 1] BeginPlay (Initial Setting)
  (bind _asbp_lsh_bphpwidget (cast `/Game/2_BP/Widget/BP_LSH_BPHPWidget` (`WidgetComponent.GetWidget` (`self.HPBar`))))
  (set `/Game/2_BP/Widget/BP_LSH_BPHPWidget.Dino_ref` self _asbp_lsh_bphpwidget)
  (set `CharacterMovementComponent.MaxWalkSpeed` (* 150.0 (`self.speedStat`)) (`self.CharacterMovement`))
  (set `self.HP` (`KismetMathLibrary.FTrunc` (* 30.0 (`self.defenceStat`))))
  (`self.SpecialSkillEffectMaker`)
  (`self.buffSkillEffectMaker`)
  (bind _returnvalue (`|CreateWidget` "/Game/2_BP/Widget/inBattle/BP_InGameBattleWidget.BP_InGameBattleWidget_C"))
  (`UserWidget.AddToViewport` _returnvalue 0))

(event `Key|Five`
  (params (Key :type "Key Structure"))
  ;[0.07669 0.9741 1] BeginPlay (Initial Setting)
  (:`Pressed`
    (`/Game/2_BP/Widget/inBattle/BP_InGameBattleWidget.hit` (stale `self.ReceiveBeginPlay` _returnvalue))))

(event `fireEffectServer`
  (`self.fireEffectMulticast`))

(event `self.ReceiveAnyDamage`
  (params (Damage :type "Float (single-precision)") (DamageType :type "DamageType Object Reference") (InstigatedBy :type "Controller Object Reference") (DamageCauser :type "Actor Object Reference"))
  (bind _returnvalue (`GameplayStatics.GetObjectClass` DamageType))
  ;[1 1 1] Apply Damage & Die
  (if (== _returnvalue "/Game/2_BP/DamageType/DT_Fire.DT_Fire_C")
    (if (not (`self.noDamageTime`))
      (`KismetSystemLibrary.PrintString` "fire!!!!!!!" false)
      (set `self.TRexHP` (- (`self.TRexHP`) Damage))
      (set `self.noDamageTime` true)
      (`KismetSystemLibrary.Delay` 0.5)
      (set `self.noDamageTime` false))
    (elif (== _returnvalue "/Game/2_BP/DamageType/DT_Laser.DT_Laser_C")
      (`KismetSystemLibrary.PrintString` "tailATK hit!!!" false :!label _label)
      (if (`self.isNoHit`)
        (set `self.TRexHP` (- (`self.TRexHP`) Damage))
        (`self.playHitSound`)
        (set `self.isNoHit` false)
        (`self.hitEffectServer`))
      (elif (== _returnvalue "/Game/2_BP/DamageType/DT_Ice.DT_Ice_C")
        (if (`self.noDamageTime`)
          _
          (elif (`self.isNoHit`)
            (`KismetSystemLibrary.PrintString` "cold!!!!!" false)
            (set `self.TRexHP` (- (`self.TRexHP`) Damage))
            (set `self.isNoHit` false)
            (set `self.noDamageTime` true)
            (set `CharacterMovementComponent.MaxWalkSpeed` (* 50.0 (`self.speedStat`)) (`self.CharacterMovement`))
            (`KismetSystemLibrary.Delay` 0.5)
            (set `self.isNoHit` true)
            (`KismetSystemLibrary.Delay` 5.0)
            (set `self.noDamageTime` false)
            (set `CharacterMovementComponent.MaxWalkSpeed` (* 150.0 (`self.speedStat`)) (`self.CharacterMovement`))))
        (elif (== _returnvalue "/Game/2_BP/DamageType/DT_Tail.DT_Tail_C")
          (goto _label)
          (elif (== _returnvalue "/Game/2_BP/DamageType/DT_Bite.DT_Bite_C")
            (goto _label)
            (elif (== _returnvalue "/Game/2_BP/DamageType/DT_Roar.DT_Roar_C")
              (goto _label))))))))

(event `fireEffectMulticast`
  (`GameplayStatics.SpawnEmitterAttached` "/Game/StarterContent/Particles/P_Fire.P_Fire" (`self.CapsuleComponent`) "None" (0.0 110.0 0.0)))

(event `self.ReceiveHit`
  (params (MyComp :type "PrimitiveComponent Object Reference") (Other :type "Actor Object Reference") (OtherComp :type "PrimitiveComponent Object Reference") (bSelfMoved :type Boolean) (HitLocation :type "Vector Structure") (HitNormal :type "Vector Structure") (NormalImpulse :type "Vector Structure") (Hit :type "HitResult Structure (by ref)"))
  ;[0.144 1 0] 임시 저장소
)

(event `TRexTailAttack_1`
  (params (Val :type "InputActionValue Structure (by ref)"))
  ;[1 0.6315 0.1256] I
)

(event `hitEffectServer`
  (`self.hitEffectMulticast`))

(event `taliATK2`
  ;[1 0.6315 0.1256] I
)

(event `tailatak`
  ;[1 0.6315 0.1256] I
  (`self.taliATK2`))

(event `EnhancedInput|/Game/7_MISC/Input/IA_TRexLook`
  (params (ActionValue :type "Vector2D Structure") (ElapsedSeconds :type "Float (double-precision)") (TriggeredSeconds :type "Float (double-precision)") (InputAction :type "InputAction Object Reference" :default "/Game/7_MISC/Input/IA_TRexLook.IA_TRexLook"))
  ;[0.1665 0.08562 0.2292] In Place Turn
  (:`Triggered`
    (if (== (`KismetMathLibrary.VSize` (`MovementComponent.Velocity` (`self.CharacterMovement`))) 0.0)
      (`|ExecutionSequence`
        (:`then_0`
          (if (>= ActionValue_X 0.7)
            (set `self.bTurnRight` true)
            (set `self.bTurnLeft` false)
            (else
              (set `self.bTurnRight` false))))
        (:`then_1`
          (if (<= ActionValue_X -0.7)
            (set `self.bTurnLeft` true)
            (set `self.bTurnRight` false)
            (else
              (set `self.bTurnLeft` false)))))
      (else
        (set `self.bTurnLeft` false)
        (set `self.bTurnRight` false)))))

(event `hitEffectMulticast`
  (if (<= (`self.TRexHP`) 0.0)
    ;[0 0.06098 1] Die
    (`GameplayStatics.PlayWorldCameraShake` "/Game/2_BP/CameraShaking/BP_GetHit.BP_GetHit_C" (`self.K2_GetActorLocation`) 0.0 2000.0)
    (`SkeletalMeshComponent.PlayAnimation` (`self.Mesh`) "/Game/7_MISC/Animation/BlueTRex/BS/BlueTRex_A_012_TRexSue_Die_Anim.BlueTRex_A_012_TRexSue_Die_Anim" false)
    (else
      ;[1 0.304 0.6201] Damage
      (set `CharacterMovementComponent.MaxWalkSpeed` 0.0 (`self.CharacterMovement`))
      (set `self.bUseControllerRotationYaw` false)
      (`KismetSystemLibrary.Delay` 1.0)
      (set `self.isNoHit` true))))

(event `EnhancedInput|/Game/7_MISC/Input/IA_TailAttack`
  (params (ActionValue :type Boolean) (ElapsedSeconds :type "Float (double-precision)") (TriggeredSeconds :type "Float (double-precision)") (InputAction :type "InputAction Object Reference" :default "/Game/7_MISC/Input/IA_TailAttack.IA_TailAttack"))
  ;[1 0.6308 0.1248] TailAttack Practice
  (:`Started`
    (`self.tailatak`)))

(event `Key|Zero`
  (params (Key :type "Key Structure"))
  (:`Pressed`
    (`self.flameThrowerServer`)))

(event `flameThrowerServer`
  (`self.flameThrowerMulticast`))

(event `flameThrowerMulticast`
  (bind _iceattacklocvector (`self.iceAttackLocVector`))
  (bind _charactermovement (`self.CharacterMovement`))
  (bind (_returnvalue_roll _returnvalue_pitch _returnvalue_yaw) (`KismetMathLibrary.BreakRotator` (`KismetMathLibrary.Conv_VectorToRotator` (`self.GetActorForwardVector`))))
  (bind (_returnvalue_roll_2 _returnvalue_pitch_2 _returnvalue_yaw_2) (`KismetMathLibrary.BreakRotator` (`KismetMathLibrary.Conv_VectorToRotator` (`self.GetActorForwardVector`))))
  (if (`self.SpecialCoolTime`)
    (`KismetSystemLibrary.PrintString` "coolTime!!!!" false true (struct :`R` 1.0 :`G` 0.960876 :`A` 1.0))
    (else
      (set `self.SpecialCoolTime` true)
      (switch `int` (`self.SpecialSkill`)
        (:`Default`
          (`|ExecutionSequence` :!label _label_2
            (:`then_0`
              (`|PlayMontage` (`self.TRexBody`) "/Game/7_MISC/Animation/BlueTRex/Skill/FireBreath/BlueTRex_014_ck2_Anim_FireBreath_Montage3.BlueTRex_014_ck2_Anim_FireBreath_Montage3" 1.0 0.0 "None"
                (:`then`
                  (bind (_direction _firebreathaim) (`Timeline|FireBreathAim` :!label _label_3)
                    (:`Update`
                      (set `SpringArmComponent.TargetArmLength` (`KismetMathLibrary.Lerp` 600.0 350.0 _firebreathaim) (`self.SpringArm`)))))
                (:`OnCompleted`
                  (goto _label_3 :!via `Reverse`))))
            (:`then_1`
              ;[1 0.5652 0.2997] 화염방사 스킬
              (`ActorComponent.ToggleActive` (`self.SkillNiaEffect`))
              (set `self.bFlameOnOff` true)
              (`self.flameProjectileSpawner`)
              (`KismetSystemLibrary.Delay` 5.0)
              (`ActorComponent.Deactivate` (`self.SkillNiaEffect`))
              (set `self.bFlameOnOff` false)
              (`KismetSystemLibrary.Delay` 5.0)
              (set `self.SpecialCoolTime` false)
              (`KismetSystemLibrary.PrintString` "coolDown!!!!!!" false :!label _label_4))))
        (:`0`
          (goto _label_2))
        (:`1`
          ;[0.2462 1 0.9216] 레이저 스킬
          (set `self.bLaserBeam` true))
        (:`2`
          ;[0.3265 0.6439 1] 얼음 스킬
          (`|PlayMontage` (`self.TRexBody`) "/Game/7_MISC/Animation/BlueTRex/Skill/ICEStalagmite/BlueTRex_IceStalagmite_Montage.BlueTRex_IceStalagmite_Montage"
            (:`then`
              (set `self.bICEStalagmite` true)
              (set `CharacterMovementComponent.MaxWalkSpeed` 0.0 _charactermovement))
            (:`OnCompleted`
              (set `self.bICEStalagmite` false)
              (set `CharacterMovementComponent.MaxWalkSpeed` 600.0 _charactermovement))
            (:`OnNotifyBegin`
              (`ActorComponent.ToggleActive` (`self.SkillEmitterEffect2`))
              (`SceneComponent.K2_SetWorldLocation` (`self.SkillEmitterEffect2`) (`SceneComponent.GetSocketLocation` (`self.TRexBody`) "bn_RightFootMiddle2_63") false false)
              (`SceneComponent.K2_SetWorldRotation` (`self.SkillEmitterEffect2`) (`KismetMathLibrary.MakeRotator` _returnvalue_roll _returnvalue_pitch (+ _returnvalue_yaw -90.0)) false false)
              (`KismetSystemLibrary.Delay` 0.2)
              (`ActorComponent.ToggleActive` (`self.SkillEmitterEffect`))
              (`SceneComponent.K2_SetWorldLocation` (`self.SkillEmitterEffect`) (`SceneComponent.GetSocketLocation` (`self.TRexBody`) "bn_RightFootMiddle2_63") false false)
              (`SceneComponent.K2_SetWorldRotation` (`self.SkillEmitterEffect`) (`KismetMathLibrary.MakeRotator` _returnvalue_roll_2 _returnvalue_pitch_2 (+ _returnvalue_yaw_2 -90.0)) false false)
              (set `self.iceAttackFwdVector` (`self.GetActorForwardVector`))
              (set `self.iceAttackLocVector` (`SceneComponent.GetSocketLocation` (`self.TRexBody`) "bn_RightFootMiddle2_63"))
              (bind (_direction_2 _newtrack_1) (`Timeline|iceCollision` :!via `PlayFromStart`)
                (:`Update`
                  (for _index (range 3)
                    (bind (_outhit _returnvalue) (`KismetSystemLibrary.BoxTraceSingleForObjects` :`Start` _iceattacklocvector :`End` (+ _iceattacklocvector (* (`KismetMathLibrary.GreaterGreater_VectorRotator` (`self.iceAttackFwdVector`) (`KismetMathLibrary.MakeRotator` 0.0 0.0 (`KismetMathLibrary.Conv_IntToDouble` (- (* _index 20) 20)))) (* _newtrack_1 1000.0))) :`HalfSize` (50.0 50.0 50.0) :`ObjectTypes` (`|MakeArray` "ObjectTypeQuery3" :!type "EObjectTypeQuery Enum") :`DrawDebugType` "ForOneFrame" :`DrawTime` (`self.GetActorTickInterval`)))
                    (if _returnvalue
                      (`GameplayStatics.ApplyDamage` (`.HitActor` (`GameplayStatics.BreakHitResult` _outhit)) (* (`self.powerStat`) 1.0) null null "/Game/2_BP/DamageType/DT_Ice.DT_Ice_C")
                      (`KismetSystemLibrary.PrintString` "coolDown!!!!!!" false))))
                (:`Finished`
                  (`KismetSystemLibrary.Delay` 5.0)
                  (set `self.SpecialCoolTime` false))))))))))

(event `TailAttackEnd`
  ;[0.07619 0.3325 0.07036] Notify_TailAttackEnd Call Function
  (set `self.TailAttack` false)
  (set `CharacterMovementComponent.MaxWalkSpeed` (* 150.0 (`self.speedStat`)) (`self.CharacterMovement`))
  (`SkeletalMeshComponent.SetAnimationMode` (`self.Mesh`) "AnimationBlueprint")
  (set `self.bUseControllerRotationYaw` true))

(event `GetHitEnd`
  ;[0.07619 0.3325 0.07036] Notify_GetHitEnd
  (set `CharacterMovementComponent.MaxWalkSpeed` (* 150.0 (`self.speedStat`)) (`self.CharacterMovement`))
  (`SkeletalMeshComponent.SetAnimationMode` (`self.Mesh`) "AnimationBlueprint")
  (set `self.bUseControllerRotationYaw` true))

(event `LaserBeam_Start`
  (bind _trexbody (`self.TRexBody`))
  (bind _returnvalue (`SceneComponent.GetSocketLocation` _trexbody "bn_Tongue3_14"))
  ;[0.2462 1 0.9216] Notify_LaserBeam_Start
  (set `CharacterMovementComponent.MaxWalkSpeed` 0.0 (`self.CharacterMovement`))
  (set `self.bUseControllerRotationYaw` false)
  ;[0.2462 1 0.9216] 레이저 스킬
  (`ActorComponent.ToggleActive` (`self.SkillNiaEffect`))
  (bind (_outhit _returnvalue_2) (`KismetSystemLibrary.SphereTraceSingleForObjects` :`Start` _returnvalue :`End` (+ _returnvalue (* (`SceneComponent.GetRightVector` _trexbody) 800.0)) :`Radius` 20.0 :`ObjectTypes` (`|MakeArray` "ObjectTypeQuery3" "ObjectTypeQuery9" "ObjectTypeQuery10" :!type "EObjectTypeQuery Enum") :`DrawDebugType` "ForDuration"))
  (`|ExecutionSequence`
    (:`then_0`
      (if _returnvalue_2
        (`GameplayStatics.ApplyDamage` (`.HitActor` (`GameplayStatics.BreakHitResult` _outhit)) (* (`self.powerStat`) 5.0) null null "/Game/2_BP/DamageType/DT_Laser.DT_Laser_C")))
    (:`then_1`
      (`KismetSystemLibrary.Delay` 5.0)
      (set `self.SpecialCoolTime` false)
      (goto _label_4))))

(event `flameProjectileSpawner`
  ;[1 1 1] 화염방사 충돌체 생성
  (if (`self.bFlameOnOff`) :!label _label_5
    (`|SpawnActorFromClass` "/Game/2_BP/BP_FlameProjectile.BP_FlameProjectile_C" (`KismetMathLibrary.MakeTransform` (`SceneComponent.GetSocketLocation` (`self.TRexBody`) "bn_Jaw_11") (struct) (10.0 10.0 10.0)) "AlwaysSpawn" "MultiplyWithRoot" self null)
    (`KismetSystemLibrary.Delay` 0.2)
    (goto _label_5)))

(event `LaserBeam_End`
  ;[0.2462 1 0.9216] Notify_LaserBeam_End
  (set `self.bLaserBeam` false)
  (set `CharacterMovementComponent.MaxWalkSpeed` (* 150.0 (`self.speedStat`)) (`self.CharacterMovement`))
  (set `self.bUseControllerRotationYaw` true))

(event `Key|Two`
  (params (Key :type "Key Structure"))
  ;[1 0 0.1714] Bite
  (:`Pressed`
    (`self.BiteAttackServer`)))

(event `BiteAttackServer`
  ;[1 0 0.1714] Bite
  (`self.BiteAttackMulticast`))

(event `BiteAttackMulticast`
  ;[1 0 0.1714] Bite
  (if (not (`self.bBite`))
    (set `self.bBite` true)
    (`|PlayMontage` (`self.TRexBody`) "/Game/7_MISC/Animation/BlueTRex/Skill/Bite/BlueTRex_Attack_biteShaking_2_Montage.BlueTRex_Attack_biteShaking_2_Montage"
      (:`OnCompleted`
        (set `self.bBite` false)))))

(event `Key|Three`
  (params (Key :type "Key Structure"))
  ;[1 0.4233 0] Roar
  (:`Pressed`
    (`self.RoarAttack_Sever`)))

(event `RoarAttack_Sever`
  ;[1 0.4233 0] Roar
  (`self.Roar_Attack_Multicast`))

(event `Roar_Attack_Multicast`
  ;[1 0.4233 0] Roar
  (set `self.bRoar` true)
  (set `CharacterMovementComponent.MaxWalkSpeed` 0.0 (`self.CharacterMovement`))
  (set `self.bUseControllerRotationYaw` false))

(event `Roar_Attack_End`
  ;[1 0.4233 0] Roar
  (set `self.bRoar` false)
  (set `CharacterMovementComponent.MaxWalkSpeed` 600.0 (`self.CharacterMovement`))
  (set `self.bUseControllerRotationYaw` true))

(event `BuffSkillMulticast`
  (bind _tempstat (`self.tempStat`))
  ;[1 0.8963 0.3185] buff Skill
  (if (`self.BuffCoolTime`)
    (`KismetSystemLibrary.PrintString` "buff cool time !!!!!" false)
    (else
      (set `self.BuffCoolTime` true)
      (switch `int` (`self.BuffSkill`)
        (:`0`
          (bind _output_get (set `self.tempStat` (`self.powerStat`)))
          (set `self.powerStat` (+ _output_get 3.0)))
        (:`1`
          (bind _output_get_2 (set `self.tempStat` (`self.defenceStat`)))
          (set `self.defenceStat` (+ _output_get_2 3.0)))
        (:`2`
          (bind _output_get_3 (set `self.tempStat` (`self.speedStat`)))
          (set `self.speedStat` (+ _output_get_3 3.0))
          (set `CharacterMovementComponent.MaxWalkSpeed` (* 150.0 (`self.speedStat`)) (`self.CharacterMovement`))))
      (`ActorComponent.SetActive` (`self.BuffEffect`) true false)
      (`KismetSystemLibrary.Delay` 6.0)
      (switch `int` (`self.BuffSkill`)
        (:`0`
          (set `self.powerStat` _tempstat))
        (:`1`
          (set `self.defenceStat` _tempstat))
        (:`2`
          (set `self.speedStat` _tempstat)
          (set `CharacterMovementComponent.MaxWalkSpeed` (* 150.0 (`self.speedStat`)) (`self.CharacterMovement`))))
      (`ActorComponent.SetActive` (`self.BuffEffect`) false false)
      (`KismetSystemLibrary.Delay` 10.0)
      (set `self.BuffCoolTime` false))))

(event `Key|Nine`
  (params (Key :type "Key Structure"))
  ;[1 0.8963 0.3185] Buff Practice
  (:`Pressed`
    (`self.BuffSkillServer`)))

(event `BuffSkillServer`
  ;[1 0.8963 0.3185] Buff Practice
  (`self.BuffSkillMulticast`))

(fn `buffSkillEffectMaker`
  (switch `int` (`self.BuffSkill`)
    (:`Default`
      (bind _returnvalue (`NiagaraFunctionLibrary.SpawnSystemAttached` "/Game/5_FX/NS_PowerBuffEffect.NS_PowerBuffEffect" (`self.CapsuleComponent`) "None" (0.0 -0.0 -88.0) (struct :`Yaw` 90.0) "KeepRelativeOffset" false false :!label _label))
      (set `self.BuffEffect` _returnvalue))
    (:`0`
      (goto _label))
    (:`1`
      (bind _returnvalue_2 (`NiagaraFunctionLibrary.SpawnSystemAttached` "/Game/5_FX/NS_HealBuffEffect.NS_HealBuffEffect" (`self.CapsuleComponent`) "None" (0.0 -0.0 -88.0) (struct) "KeepRelativeOffset" false false))
      (set `self.BuffEffect` _returnvalue_2))
    (:`2`
      (bind _returnvalue_3 (`NiagaraFunctionLibrary.SpawnSystemAttached` "/Game/5_FX/NS_SpeedBuffEffect.NS_SpeedBuffEffect" (`self.CapsuleComponent`) "None" (0.0 -0.0 -88.0) (struct) "KeepRelativeOffset" false false))
      (set `self.BuffEffect` _returnvalue_3))))

(fn `playHitSound`
  (locals (sound2Play :type "SoundBase Object Reference"))
  (switch `int` (`KismetMathLibrary.RandomIntegerInRange` 0 2)
    (:`0`
      (set `local.sound2Play` "/Game/8_SOUND/DinoHitSound/Smash_Hit_Sound_Effects_HD__mp3cut_net_.Smash_Hit_Sound_Effects_HD__mp3cut_net_"))
    (:`1`
      (set `local.sound2Play` "/Game/8_SOUND/DinoHitSound/Smash_Hit_Sound_Effects_HD__mp3cut_net___1_.Smash_Hit_Sound_Effects_HD__mp3cut_net___1_"))
    (:`2`
      (set `local.sound2Play` "/Game/8_SOUND/DinoHitSound/Smash_Hit_Sound_Effects_HD__mp3cut_net___2_.Smash_Hit_Sound_Effects_HD__mp3cut_net___2_")))
  (`GameplayStatics.PlaySoundAtLocation` (`local.sound2Play`) (`self.K2_GetActorLocation`) (struct) 1.0 1.0 0.0 "/Game/8_SOUND/PlayerSoundAttenuation.PlayerSoundAttenuation" null null null))

(fn `SpecialSkillEffectMaker`
  (switch `int` (`self.SpecialSkill`)
    (:`0`
      (bind _returnvalue (`NiagaraFunctionLibrary.SpawnSystemAttached` "/Game/DragonFlameFX/FX/NS_DragonFlame_Fire1.NS_DragonFlame_Fire1" (`self.TRexBody`) "bn_Jaw_11" (0.0 0.0 0.0) (struct :`Pitch` -20.0) "KeepRelativeOffset" false false))
      (set `self.SkillNiaEffect` _returnvalue))
    (:`1`
      (bind _returnvalue_2 (`NiagaraFunctionLibrary.SpawnSystemAttached` "/Game/5_FX/VFX_Laser1.VFX_Laser1" (`self.TRexBody`) "LaserBeam_Point" (0.0 0.0 0.0) (`KismetMathLibrary.Conv_VectorToRotator` (* (`self.GetActorForwardVector`) (-1.0 0.0 0.0))) "KeepRelativeOffset" false false))
      (set `self.SkillNiaEffect` _returnvalue_2))
    (:`2`
      (bind _returnvalue_3 (`GameplayStatics.SpawnEmitterAtLocation` "/Game/5_FX/P_IceGroundAttack17.P_IceGroundAttack17" (0.0 0.0 0.0) (struct) (1.0 1.5 1.5) false "None" false))
      (set `self.SkillEmitterEffect` _returnvalue_3)
      (bind _returnvalue_4 (`GameplayStatics.SpawnEmitterAtLocation` "/Game/5_FX/P_IceGroundAttack171.P_IceGroundAttack171" (0.0 0.0 0.0) (struct) (1.0 0.5 0.5) false "None" false))
      (set `self.SkillEmitterEffect2` _returnvalue_4))))

(fn `UserConstructionScript`
  (`SceneComponent.K2_AttachToComponent` (`self.Tail`) (`self.TRexBody`) "bn_Tail05_71" "KeepRelative" "KeepRelative" "KeepRelative" true)
  (`SceneComponent.K2_AttachToComponent` (`self.UpperBody`) (`self.TRexBody`) "bn_Neck_7" "KeepRelative" "KeepRelative" "KeepRelative" true)
  (`SceneComponent.K2_AttachToComponent` (`self.Head`) (`self.TRexBody`) "bn_Head_10" "KeepRelative" "KeepRelative" "KeepRelative" true))