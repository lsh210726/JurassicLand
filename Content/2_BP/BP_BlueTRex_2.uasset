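; Blue T-Rex child Blueprint that tracks HP, stages a camera and animation sequence, and forwards tail attacks to its parent.
; Damage lowers and prints HP, then blocks further hits for one second.
; After a BeginPlay delay, the TRexEye camera snaps to the tail-attack spring arm while the death animation plays, then returns to its eye arm.
; The 0 key fires two custom events that both call the parent's tail attack.
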(event `self.ReceiveAnyDamage`
  (params (Damage :type "Float (single-precision)") (DamageType :type "DamageType Object Reference") (InstigatedBy :type "Controller Object Reference") (DamageCauser :type "Actor Object Reference"))
  (if (`self.isNoHit`)
    (bind _output_get (set `self.HP` (- (`self.HP`) Damage)))
    (`KismetSystemLibrary.PrintString` (`KismetStringLibrary.Conv_IntToString` _output_get))
    (set `self.isNoHit` false)
    (`KismetSystemLibrary.Delay` 1.0)
    (set `self.isNoHit` true)))

(event `self.ReceiveBeginPlay`
  (bind _trexeye (`self.TRexEye`))
  (`KismetSystemLibrary.Delay` 3.0)
  (`SceneComponent.K2_AttachToComponent` (`self.TRexEye`) (`self.TailAttackSpringArm`) "None" "SnapToTarget" "SnapToTarget" "SnapToTarget" true)
  (`SceneComponent.K2_SetRelativeRotation` _trexeye (struct :`Yaw` -25.3) false false)
  (set `CameraComponent.FieldOfView` 90.0 _trexeye)
  (`SkeletalMeshComponent.PlayAnimation` (`self.Mesh`) "/Game/7_MISC/Animation/BlueTRex/BS/BlueTRex_A_012_TRexSue_Die_Anim.BlueTRex_A_012_TRexSue_Die_Anim" false)
  (`KismetSystemLibrary.Delay` 6.0)
  (`SceneComponent.K2_AttachToComponent` (`self.TRexEye`) (`self.TRexEyeArm`) "None" "SnapToTarget" "SnapToTarget" "SnapToTarget" true))

(event `self.ReceiveHit`
  (params (MyComp :type "PrimitiveComponent Object Reference") (Other :type "Actor Object Reference") (OtherComp :type "PrimitiveComponent Object Reference") (bSelfMoved :type Boolean) (HitLocation :type "Vector Structure") (HitNormal :type "Vector Structure") (NormalImpulse :type "Vector Structure") (Hit :type "HitResult Structure (by ref)")))

(event `self.TRexTailAttack`
  (params (Val :type "InputActionValue Structure (by ref)"))
  (`parent.TRexTailAttack` Val :!label _label))

(event `taliATK2`
  (goto _label))

(event `tailatak`
  (goto _label))

(event `Key|Zero`
  (params (Key :type "Key Structure"))
  (:`Pressed`
    (`self.tailatak`)
    (`self.taliATK2`)))

(fn `UserConstructionScript`)