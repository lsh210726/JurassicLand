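; BP_FlameProjectile is a short-lived fire attack projectile spawned by BP_BlueTRex.
; It sets a brief lifespan on begin play and grows its actor scale a little every tick.
; On overlap with anything but its owner, it applies fire damage scaled by the owning T-Rex's PowerStat and triggers that T-Rex's hit marker, printing a debug message if the owner cast fails.
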(event `self.ReceiveBeginPlay`
  (`self.SetLifeSpan` 1.0))

(event `self.ReceiveTick`
  (params (DeltaSeconds :type "Float (single-precision)"))
  (`self.SetActorScale3D` (`self.scale`))
  (set `self.scale` (+ (`self.scale`) 0.01)))

(event `self.ReceiveActorBeginOverlap`
  (params (OtherActor :type "Actor Object Reference"))
  (bind _returnvalue (`self.GetOwner`))
  (if (!= OtherActor _returnvalue)
    (bind _asbp_blue_trex (cast `/Game/2_BP/BP_BlueTRex` _returnvalue)
      (:`then`
        (`GameplayStatics.ApplyDamage` OtherActor (* (`/Game/2_BP/BP_BlueTRex.powerStat` _asbp_blue_trex) 1.0) null (`self.Instigator`) "/Game/2_BP/DamageType/DT_Fire.DT_Fire_C")
        (bind _asbp_blue_trex_2 (cast `/Game/2_BP/BP_BlueTRex` (`self.GetOwner`)))
        (`/Game/2_BP/BP_BlueTRex.HitMarkerMaker` _asbp_blue_trex_2))
      (:`CastFailed`
        (`KismetSystemLibrary.PrintString` "fire atk cast fail !!!!!!" false)))))

(fn `UserConstructionScript`)