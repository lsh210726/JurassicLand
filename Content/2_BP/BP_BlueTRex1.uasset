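; Playable blue T-Rex character with a C++-backed tail attack, a special skill, a buff and hit/death reactions.
; BeginPlay applies stats, links the HP widget and pre-spawns effects for the selected skills.
; Input triggers Server-to-Multicast event chains with delay-based cooldowns: flamethrower projectiles, laser sphere trace or timeline-driven three-way ice box traces, while buffs only toggle Niagara effects.
; AnyDamage reduces TRexHP behind an IsNoHit gate, then multicasts hit or death feedback.
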(event `self.ReceiveTick`
  (params (DeltaSeconds :type "Float (single-precision)")))

(event `self.ReceiveBeginPlay`
  ;[0.07669 0.9741 1] BeginPlay (Initial Setting)
  (bind _asbp_lsh_bphpwidget (cast `/Game/2_BP/Widget/BP_LSH_BPHPWidget` (`WidgetComponent.GetWidget` (`self.HPBar`))))
  (set `/Game/2_BP/Widget/BP_LSH_BPHPWidget.Dino_ref` self _asbp_lsh_bphpwidget)
  (set `CharacterMovementComponent.MaxWalkSpeed` (* 150.0 (`self.speedStat`)) (`self.CharacterMovement`))
  (set `self.HP` (`KismetMathLibrary.FTrunc` (* 30.0 (`self.defenceStat`))))
  (`self.SpecialSkillEffectMaker`)
  (switch `int` (`self.BuffSkill`)
    (:`Default`
      (bind _returnvalue (`NiagaraFunctionLibrary.SpawnSystemAttached` "/Game/5_FX/NS_PowerBuffEffect.NS_PowerBuffEffect" (`self.CapsuleComponent`) "None" (0.0 -0.0 -88.0) (struct :`Yaw` 90.0) "KeepRelativeOffset" false false :!label _label))
      (set `self.BuffEffect` _returnvalue))
    (:`0`
      (goto _label))
    (:`1`
      (bind _returnvalue_2 (`NiagaraFunctionLibrary.SpawnSystemAttached` "/Game/5_FX/NS_HealBuffEffect.NS_HealBuffEffect" (`self.CapsuleComponent`) "None" (0.0 -0.0 -88.0) (struct) "KeepRelativeOffset" false false))
      (set `self.BuffEffect` _returnvalue_2))
    (:`2`
      (bind _returnvalue_3 (`NiagaraFunctionLibrary.SpawnSystemAttached` "/Game/5_FX/NS_SpeedBuffEffect.NS_SpeedBuffEffect" (`self.CapsuleComponent`) "None" (0.0 -0.0 -88.0) (struct) "KeepRelativeOffset" false false))
      (set `self.BuffEffect` _returnvalue_3))))

(event `self.ReceiveAnyDamage`
  (params (Damage :type "Float (single-precision)") (DamageType :type "DamageType Object Reference") (InstigatedBy :type "Controller Object Reference") (DamageCauser :type "Actor Object Reference"))
  ;[1 1 1] Apply Damage & Die
  (if (`self.isNoHit`)
    (set `self.TRexHP` (- (`self.TRexHP`) Damage))
    (`self.playHitSound`)
    (set `self.isNoHit` false)
    (`self.hitEffectServer`)))

(event `self.ReceiveHit`
  (params (MyComp :type "PrimitiveComponent Object Reference") (Other :type "Actor Object Reference") (OtherComp :type "PrimitiveComponent Object Reference") (bSelfMoved :type Boolean) (HitLocation :type "Vector Structure") (HitNormal :type "Vector Structure") (NormalImpulse :type "Vector Structure") (Hit :type "HitResult Structure (by ref)"))
  ;[0.144 1 0] 임시 저장소
)

(event `self.TRexTailAttack`
  (params (Val :type "InputActionValue Structure (by ref)"))
  ;[1 0.6315 0.1256] TailAttack C++ Code Native
  (`parent.TRexTailAttack` Val :!label _label_2))

(event `hitEffectServer`
  (`self.hitEffectMulticast`))

(event `taliATK2`
  ;[1 0.6315 0.1256] TailAttack C++ Code Native
  (goto _label_2))

(event `tailatak`
  ;[1 0.6315 0.1256] TailAttack C++ Code Native
  (`self.taliATK2`))

(event `hitEffectMulticast`
  (if (<= (`self.TRexHP`) 0.0)
    ;[0 0.06098 1] Die
    (`GameplayStatics.PlayWorldCameraShake` "/Game/2_BP/CameraShaking/BP_GetHit.BP_GetHit_C" (`self.K2_GetActorLocation`) 0.0 2000.0)
    (`SkeletalMeshComponent.PlayAnimation` (`self.Mesh`) "/Game/7_MISC/Animation/BlueTRex/BS/BlueTRex_A_012_TRexSue_Die_Anim.BlueTRex_A_012_TRexSue_Die_Anim" false)
    (else
      ;[1 0.304 0.6201] Damage
      (set `CharacterMovementComponent.MaxWalkSpeed` 0.0 (`self.CharacterMovement`))
      (set `self.bUseControllerRotationYaw` false)
      (`KismetSystemLibrary.Delay` 1.0)
      (set `self.isNoHit` true))))

(event `EnhancedInput|/Game/7_MISC/Input/IA_TailAttack`
  (params (ActionValue :type Boolean) (ElapsedSeconds :type "Float (double-precision)") (TriggeredSeconds :type "Float (double-precision)") (InputAction :type "InputAction Object Reference" :default "/Game/7_MISC/Input/IA_TailAttack.IA_TailAttack"))
  ;[1 0.6308 0.1248] Comment
  (:`Started`
    (`self.tailatak`)))

(event `flameThrowerServer`
  (`self.flameThrowerMulticast`))

(event `flameThrowerMulticast`
  (bind _trexbody (`self.TRexBody`))
  (bind _iceattacklocvector (`self.iceAttackLocVector`))
  (bind (_returnvalue_roll _returnvalue_pitch _returnvalue_yaw) (`KismetMathLibrary.BreakRotator` (`KismetMathLibrary.Conv_VectorToRotator` (`self.GetActorForwardVector`))))
  (bind _returnvalue (`SceneComponent.GetSocketLocation` _trexbody "bn_Tongue3_14"))
  (bind (_returnvalue_roll_2 _returnvalue_pitch_2 _returnvalue_yaw_2) (`KismetMathLibrary.BreakRotator` (`KismetMathLibrary.Conv_VectorToRotator` (`self.GetActorForwardVector`))))
  (if (`self.SpecialCoolTime`)
    (`KismetSystemLibrary.PrintString` "coolTime!!!!" false true (struct :`R` 1.0 :`G` 0.960876 :`A` 1.0))
    (else
      (set `self.SpecialCoolTime` true)
      (switch `int` (`self.SpecialSkill`)
        (:`Default`
          ;[1 0.5652 0.2997] 화염방사 스킬
          (`ActorComponent.ToggleActive` (`self.SkillNiaEffect`) :!label _label_3)
          (set `self.bFlameOnOff` true)
          (`self.flameProjectileSpawner`)
          (`KismetSystemLibrary.Delay` 5.0)
          (`ActorComponent.Deactivate` (`self.SkillNiaEffect`))
          (set `self.bFlameOnOff` false)
          (`KismetSystemLibrary.Delay` 5.0)
          (set `self.SpecialCoolTime` false)
          (`KismetSystemLibrary.PrintString` "coolDown!!!!!!" false :!label _label_4))
        (:`0`
          (goto _label_3))
        (:`1`
          ;[0.2454 1 0.9203] 레이저 스킬
          (`ActorComponent.ToggleActive` (`self.SkillNiaEffect`))
          (bind (_outhit _returnvalue_2) (`KismetSystemLibrary.SphereTraceSingleForObjects` :`Start` _returnvalue :`End` (+ _returnvalue (* (`SceneComponent.GetRightVector` _trexbody) 800.0)) :`Radius` 20.0 :`ObjectTypes` (`|MakeArray` "ObjectTypeQuery3" :!type "EObjectTypeQuery Enum") :`DrawDebugType` "ForDuration"))
          (if _returnvalue_2
            (`GameplayStatics.ApplyDamage` (`.HitActor` (`GameplayStatics.BreakHitResult` _outhit)) (* (`self.powerStat`) 5.0) null null "/Game/2_BP/DamageType/BP_LaserDT.BP_LaserDT_C")
            (`KismetSystemLibrary.Delay` 15.0)
            (set `self.SpecialCoolTime` false)
            (goto _label_4)))
        (:`2`
          ;[0.3265 0.6439 1] 얼음 스킬
          (`ActorComponent.ToggleActive` (`self.SkillEmitterEffect2`))
          (`SceneComponent.K2_SetWorldLocation` (`self.SkillEmitterEffect2`) (`SceneComponent.GetSocketLocation` (`self.TRexBody`) "bn_RightFootMiddle2_63") false false)
          (`SceneComponent.K2_SetWorldRotation` (`self.SkillEmitterEffect2`) (`KismetMathLibrary.MakeRotator` _returnvalue_roll _returnvalue_pitch (+ _returnvalue_yaw -90.0)) false false)
          (`KismetSystemLibrary.Delay` 0.2)
          (`ActorComponent.ToggleActive` (`self.SkillEmitterEffect`))
          (`SceneComponent.K2_SetWorldLocation` (`self.SkillEmitterEffect`) (`SceneComponent.GetSocketLocation` (`self.TRexBody`) "bn_RightFootMiddle2_63") false false)
          (`SceneComponent.K2_SetWorldRotation` (`self.SkillEmitterEffect`) (`KismetMathLibrary.MakeRotator` _returnvalue_roll_2 _returnvalue_pitch_2 (+ _returnvalue_yaw_2 -90.0)) false false)
          (set `self.iceAttackFwdVector` (`self.GetActorForwardVector`))
          (set `self.iceAttackLocVector` (`SceneComponent.GetSocketLocation` (`self.TRexBody`) "bn_RightFootMiddle2_63"))
          (bind (_direction _newtrack_1) (`Timeline|iceCollision` :!via `PlayFromStart`)
            (:`Update`
              (for _index (range 3)
                (bind (_outhit_2 _returnvalue_3) (`KismetSystemLibrary.BoxTraceSingleForObjects` :`Start` _iceattacklocvector :`End` (+ _iceattacklocvector (* (`KismetMathLibrary.GreaterGreater_VectorRotator` (`self.iceAttackFwdVector`) (`KismetMathLibrary.MakeRotator` 0.0 0.0 (`KismetMathLibrary.Conv_IntToDouble` (- (* _index 20) 20)))) (* _newtrack_1 1000.0))) :`HalfSize` (50.0 50.0 50.0) :`ObjectTypes` (`|MakeArray` "ObjectTypeQuery3" :!type "EObjectTypeQuery Enum") :`DrawDebugType` "ForOneFrame" :`DrawTime` (`self.GetActorTickInterval`)))
                (if _returnvalue_3
                  (`GameplayStatics.ApplyDamage` (`.HitActor` (`GameplayStatics.BreakHitResult` _outhit_2)) (* (`self.powerStat`) 1.0) null null "/Game/2_BP/DamageType/BP_IceDT.BP_IceDT_C")
                  (`KismetSystemLibrary.PrintString` "coolDown!!!!!!" false))))
            (:`Finished`
              (`KismetSystemLibrary.Delay` 5.0)
              (set `self.SpecialCoolTime` false))))))))

(event `TailAttackEnd`
  ;[0.07619 0.3325 0.07036] Notify_TailAttackEnd Call Function
  (set `self.TailAttack` false)
  (set `CharacterMovementComponent.MaxWalkSpeed` 600.0 (`self.CharacterMovement`))
  (`SkeletalMeshComponent.SetAnimationMode` (`self.Mesh`) "AnimationBlueprint")
  (set `self.bUseControllerRotationYaw` true))

(event `GetHitEnd`
  ;[0.07619 0.3325 0.07036] Notify_GetHitEnd
  (set `CharacterMovementComponent.MaxWalkSpeed` 600.0 (`self.CharacterMovement`))
  (`SkeletalMeshComponent.SetAnimationMode` (`self.Mesh`) "AnimationBlueprint")
  (set `self.bUseControllerRotationYaw` true))

(event `flameProjectileSpawner`
  ;[1 1 1] 화염방사 충돌체 생성
  (if (`self.bFlameOnOff`) :!label _label_5
    (`|SpawnActorFromClass` "/Game/2_BP/BP_FlameProjectile.BP_FlameProjectile_C" (`SceneComponent.GetSocketTransform` (`self.TRexBody`) "bn_Jaw_11" "RTS_World") "Undefined" "MultiplyWithRoot" self null)
    (`KismetSystemLibrary.Delay` 0.2)
    (goto _label_5)))

(event `Key|Zero`
  (params (Key :type "Key Structure"))
  (:`Pressed`
    (`self.flameThrowerServer`)))

(event `BuffSkillServer`
  (`self.BuffSkillMulticast`))

(event `BuffSkillMulticast`
  (if (`self.BuffCoolTime`)
    (`KismetSystemLibrary.PrintString` "buff cool time !!!!!" false)
    (else
      (set `self.BuffCoolTime` true)
      (switch `int` (`self.BuffSkill`)
        (:`0`
          _)
        (:`1`
          _)
        (:`2`
          _))
      (`ActorComponent.SetActive` (`self.BuffEffect`) true false)
      (`KismetSystemLibrary.Delay` 6.0)
      (`ActorComponent.SetActive` (`self.BuffEffect`) false false)
      (`KismetSystemLibrary.Delay` 10.0)
      (set `self.BuffCoolTime` false))))

(event `Key|Nine`
  (params (Key :type "Key Structure"))
  (:`Pressed`
    (`self.BuffSkillServer`)))

(fn `playHitSound`
  (locals (sound2Play :type "SoundBase Object Reference"))
  (switch `int` (`KismetMathLibrary.RandomIntegerInRange` 0 2)
    (:`0`
      (set `local.sound2Play` "/Game/8_SOUND/DinoHitSound/Smash_Hit_Sound_Effects_HD__mp3cut_net_.Smash_Hit_Sound_Effects_HD__mp3cut_net_"))
    (:`1`
      (set `local.sound2Play` "/Game/8_SOUND/DinoHitSound/Smash_Hit_Sound_Effects_HD__mp3cut_net___1_.Smash_Hit_Sound_Effects_HD__mp3cut_net___1_"))
    (:`2`
      (set `local.sound2Play` "/Game/8_SOUND/DinoHitSound/Smash_Hit_Sound_Effects_HD__mp3cut_net___2_.Smash_Hit_Sound_Effects_HD__mp3cut_net___2_")))
  (`GameplayStatics.PlaySoundAtLocation` (`local.sound2Play`) (`self.K2_GetActorLocation`) (struct) 1.0 1.0 0.0 "/Game/8_SOUND/PlayerSoundAttenuation.PlayerSoundAttenuation" null null null))

(fn `SpecialSkillEffectMaker`
  (switch `int` (`self.SpecialSkill`)
    (:`0`
      (bind _returnvalue (`NiagaraFunctionLibrary.SpawnSystemAttached` "/Game/5_FX/NS_Fire_Flamethrower1.NS_Fire_Flamethrower1" (`self.TRexBody`) "bn_Tongue3_14" (23.0 0.0 0.0) (struct :`Yaw` 55.0 :`Roll` 23.0) "KeepRelativeOffset" false false))
      (set `self.SkillNiaEffect` _returnvalue))
    (:`1`
      (bind _returnvalue_2 (`NiagaraFunctionLibrary.SpawnSystemAttached` "/Game/5_FX/VFX_Laser1.VFX_Laser1" (`self.TRexBody`) "bn_Tongue3_14" (0.0 0.0 0.0) (struct :`Pitch` 180.0) "KeepRelativeOffset" false false))
      (set `self.SkillNiaEffect` _returnvalue_2))
    (:`2`
      (bind _returnvalue_3 (`GameplayStatics.SpawnEmitterAtLocation` "/Game/5_FX/P_IceGroundAttack17.P_IceGroundAttack17" (0.0 0.0 0.0) (struct) (1.0 1.5 1.5) false "None" false))
      (set `self.SkillEmitterEffect` _returnvalue_3)
      (bind _returnvalue_4 (`GameplayStatics.SpawnEmitterAtLocation` "/Game/5_FX/P_IceGroundAttack171.P_IceGroundAttack171" (0.0 0.0 0.0) (struct) (1.0 0.5 0.5) false "None" false))
      (set `self.SkillEmitterEffect2` _returnvalue_4))))

(fn `UserConstructionScript`)