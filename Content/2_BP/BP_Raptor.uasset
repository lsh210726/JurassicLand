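; Playable raptor character with bite, tail attack, roar and special skill inputs, relayed through server-to-multicast events.
; BeginPlay binds the HP bar, derives speed and HP from stats, and pre-spawns inactive special and buff effects chosen by skill index.
; Attacks set state flags, with tail and roar also freezing movement; the special skill only sets its cooldown flag.
; A timeline sphere-traces for a lock-on target, but the lock-on camera logic is disconnected.
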(event `self.ReceiveBeginPlay`
  ;[0.07669 0.9741 1] BeginPlay (Initial Setting)
  (bind _asbp_lsh_bphpwidget (cast `/Game/2_BP/Widget/BP_LSH_BPHPWidget` (`WidgetComponent.GetWidget` (`self.HP_Bar`))))
  (set `/Game/2_BP/Widget/BP_LSH_BPHPWidget.Dino_ref` self _asbp_lsh_bphpwidget)
  (set `CharacterMovementComponent.MaxWalkSpeed` (* 150.0 (`self.SpeedStat`)) (`self.CharacterMovement`))
  (set `self.HP` (`KismetMathLibrary.FTrunc` (* 30.0 (`self.DefenceStat`))))
  (`self.SpecialSkillEffectMaker`)
  (`self.buffSkillEffectMaker`)
  (`Timeline|Timeline_0` :!via `PlayFromStart`
    (:`Update`
      (`self.LockOnTarget`
        (:`then`)
        (:`else`
          (bind (_outhit _returnvalue) (`KismetSystemLibrary.SphereTraceSingleForObjects` (`self.K2_GetActorLocation`) (0.0 0.0 0.0) 2000.0 (`|MakeArray` "ObjectTypeQuery3" :!type "EObjectTypeQuery Enum")))
          (if _returnvalue
            (set `self.LockOnTarget` (`.HitActor` (`GameplayStatics.BreakHitResult` _outhit)))))))))

(event `EnhancedInput|/Game/7_MISC/Input/IA_SpecialSkill`
  (params (ActionValue :type Boolean) (ElapsedSeconds :type "Float (double-precision)") (TriggeredSeconds :type "Float (double-precision)") (InputAction :type "InputAction Object Reference" :default "/Game/7_MISC/Input/IA_SpecialSkill.IA_SpecialSkill"))
  (:`Started`
    (`self.flameThrowerServer`)))

(event `flameThrowerServer`
  (`self.flameThrowerMulticast`))

(event `self.ReceiveTick`
  (params (DeltaSeconds :type "Float (single-precision)")))

(event `flameThrowerMulticast`
  (if (`self.CoolTime_SpecialSkill`)
    (`KismetSystemLibrary.PrintString` "coolTime!!!!" false true (struct :`R` 1.0 :`G` 0.960876 :`A` 1.0))
    (else
      (set `self.CoolTime_SpecialSkill` true)
      (switch `int` (`self.SpecialSkill`)
        (:`Default`
          _)
        (:`0`
          _))
      (`|ExecutionSequence`))))

(event `EnhancedInput|/Game/7_MISC/Input/IA_Basic_TailAttack`
  (params (ActionValue :type Boolean) (ElapsedSeconds :type "Float (double-precision)") (TriggeredSeconds :type "Float (double-precision)") (InputAction :type "InputAction Object Reference" :default "/Game/7_MISC/Input/IA_Basic_TailAttack.IA_Basic_TailAttack"))
  ;[1 1 1] TailAttack
  (:`Started`
    (`self.TailAttack_Server`)))

(event `EnhancedInput|/Game/7_MISC/Input/IA_Basic_Bite`
  (params (ActionValue :type Boolean) (ElapsedSeconds :type "Float (double-precision)") (TriggeredSeconds :type "Float (double-precision)") (InputAction :type "InputAction Object Reference" :default "/Game/7_MISC/Input/IA_Basic_Bite.IA_Basic_Bite"))
  ;[1 1 1] BiteAttack
  (:`Started`
    (`self.BiteAttack_Server`)))

(event `TailAttack_Server`
  ;[1 1 1] TailAttack
  (`self.TailAttack_Multicast`))

(event `BiteAttack_Server`
  ;[1 1 1] BiteAttack
  (`self.BiteAttack_Multicast`))

(event `TailAttack_Multicast`
  ;[1 1 1] TailAttack
  (if (not (`self.bTailAttack`))
    (set `self.bTailAttack` true)
    (set `CharacterMovementComponent.MaxWalkSpeed` 0.0 (`self.CharacterMovement`))
    (set `self.bUseControllerRotationYaw` false)))

(event `BiteAttack_Multicast`
  ;[1 1 1] BiteAttack
  (if (not (`self.bBite`))
    (set `self.bBite` true)
    (`|PlayMontage` (`self.PlayerBody`) "/Game/7_MISC/Animation/Raptor/Skill/Raptor_Bite_Montage.Raptor_Bite_Montage"
      (:`OnCompleted`
        (if (`self.bBite`)
          (set `self.bBite` false))))))

(event `TailAttackEnd`
  ;[1 1 1] TailAttack
  (if (`self.bTailAttack`)
    (set `self.bTailAttack` false)
    (set `CharacterMovementComponent.MaxWalkSpeed` (* 150.0 (`self.speedStat`)) (`self.CharacterMovement`))
    (`SkeletalMeshComponent.SetAnimationMode` (`self.Mesh`) "AnimationBlueprint")
    (set `self.bUseControllerRotationYaw` true)))

(event `EnhancedInput|/Game/7_MISC/Input/IA_Basic_Roar`
  (params (ActionValue :type Boolean) (ElapsedSeconds :type "Float (double-precision)") (TriggeredSeconds :type "Float (double-precision)") (InputAction :type "InputAction Object Reference" :default "/Game/7_MISC/Input/IA_Basic_Roar.IA_Basic_Roar"))
  ;[1 1 1] Roar
  (:`Started`
    (`self.RoarAttack_Server`)))

(event `RoarAttack_Server`
  ;[1 1 1] Roar
  (`self.RoarAttack_Multicast`))

(event `RoarAttack_Multicast`
  ;[1 1 1] Roar
  (if (not (`self.bRoar`))
    (set `self.bRoar` true)
    (set `CharacterMovementComponent.MaxWalkSpeed` 0.0 (`self.CharacterMovement`))
    (set `self.bUseControllerRotationYaw` false)))

(event `RoarAttack_End`
  ;[1 1 1] Roar
  (if (`self.bRoar`)
    (set `self.bRoar` false)
    (set `CharacterMovementComponent.MaxWalkSpeed` 600.0 (`self.CharacterMovement`))
    (set `self.bUseControllerRotationYaw` true)))

(fn `buffSkillEffectMaker`
  (switch `int` (`self.BuffSkill`)
    (:`Default`
      (`NiagaraFunctionLibrary.SpawnSystemAttached` "/Game/5_FX/NS_PowerBuffEffect.NS_PowerBuffEffect" (`self.CapsuleComponent`) "None" (0.0 -0.0 -88.0) (struct :`Yaw` 90.0) "KeepRelativeOffset" false false :!label _label))
    (:`0`
      (goto _label))
    (:`1`
      (`NiagaraFunctionLibrary.SpawnSystemAttached` "/Game/5_FX/NS_HealBuffEffect.NS_HealBuffEffect" (`self.CapsuleComponent`) "None" (0.0 -0.0 -88.0) (struct) "KeepRelativeOffset" false false))
    (:`2`
      (`NiagaraFunctionLibrary.SpawnSystemAttached` "/Game/5_FX/NS_SpeedBuffEffect.NS_SpeedBuffEffect" (`self.CapsuleComponent`) "None" (0.0 -0.0 -88.0) (struct) "KeepRelativeOffset" false false))))

(fn `SpecialSkillEffectMaker`
  (locals (SkillNiaEffect :type "NiagaraComponent Object Reference") (SkillEmitterEffect :type "ParticleSystemComponent Object Reference") (SkillEmitterEffect2 :type "ParticleSystemComponent Object Reference"))
  (switch `int` (`self.SpecialSkill`)
    (:`0`
      (bind _returnvalue (`NiagaraFunctionLibrary.SpawnSystemAttached` "/Game/DragonFlameFX/FX/NS_DragonFlame_Fire1.NS_DragonFlame_Fire1" (`self.PlayerBody`) "Jaw" (0.0 0.0 0.0) (struct :`Pitch` -20.0) "KeepRelativeOffset" false false))
      (set `local.SkillNiaEffect` _returnvalue))
    (:`1`
      (bind _returnvalue_2 (`NiagaraFunctionLibrary.SpawnSystemAttached` "/Game/5_FX/VFX_Laser1.VFX_Laser1" (`self.PlayerBody`) "LaserBeam_Point" (0.0 0.0 0.0) (`KismetMathLibrary.Conv_VectorToRotator` (* (`SceneComponent.GetForwardVector` (`self.PlayerBody`)) (-1.0 0.0 0.0))) "KeepRelativeOffset" false false))
      (set `local.SkillNiaEffect` _returnvalue_2))
    (:`2`
      (`GameplayStatics.SpawnEmitterAtLocation` "/Game/5_FX/P_IceGroundAttack17.P_IceGroundAttack17" (0.0 0.0 0.0) (struct) (1.0 1.5 1.5) false "None" false)
      (set `local.SkillEmitterEffect` null)
      (bind _returnvalue_3 (`GameplayStatics.SpawnEmitterAtLocation` "/Game/5_FX/P_IceGroundAttack171.P_IceGroundAttack171" (0.0 0.0 0.0) (struct) (1.0 0.5 0.5) false "None" false))
      (set `local.SkillEmitterEffect2` _returnvalue_3))))

(fn `UserConstructionScript`
  (`SceneComponent.K2_AttachToComponent` (`self.PlayerTailCollision`) (`self.PlayerBody`) "Tail3" "KeepRelative" "KeepRelative" "KeepRelative" true)
  (`SceneComponent.K2_AttachToComponent` (`self.PlayerUpperBodyCollision`) (`self.PlayerBody`) "Neck" "KeepRelative" "KeepRelative" "KeepRelative" true)
  (`SceneComponent.K2_AttachToComponent` (`self.PlayerHeadCollision`) (`self.PlayerBody`) "Head" "KeepRelative" "KeepRelative" "KeepRelative" true))