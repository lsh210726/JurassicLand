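; Playable Blue T-Rex combat character with tail, bite and roar attacks, a selectable fire, laser or ice special, and a power, defence or speed buff.
; Stats scale HP, speed and skill damage; AnyDamage branches on damage type for hit reactions and ice slow.
; Inputs and animation states follow Server-to-Multicast event pairs.
; A BeginPlay sphere trace picks the lock-on target that Tick faces; skill cooldown flags are never set true here.
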(event `self.ReceiveBeginPlay`
  ;[0.07669 0.9741 1] BeginPlay (Initial Setting)
  (bind _asbp_lsh_bphpwidget (cast `/Game/2_BP/Widget/BP_LSH_BPHPWidget` (`WidgetComponent.GetWidget` (`self.HP_Bar`))))
  (set `/Game/2_BP/Widget/BP_LSH_BPHPWidget.Dino_ref` self _asbp_lsh_bphpwidget)
  (set `CharacterMovementComponent.MaxWalkSpeed` (* 150.0 (`self.SpeedStat`)) (`self.CharacterMovement`))
  (set `self.State_HP` (`KismetMathLibrary.Conv_IntToDouble` (`KismetMathLibrary.FTrunc` (* 30.0 (`self.DefenceStat`)))))
  (`self.SpecialSkillEffectMaker`)
  (`self.buffSkillEffectMaker`)
  (`Timeline|Timeline_0` :!via `PlayFromStart`
    (:`Update`
      (`self.LockOnTarget`
        (:`then`)
        (:`else`
          (bind (_outhit _returnvalue) (`KismetSystemLibrary.SphereTraceSingleForObjects` (`self.K2_GetActorLocation`) (0.0 0.0 0.0) 2000.0 (`|MakeArray` "ObjectTypeQuery3" :!type "EObjectTypeQuery Enum")))
          (if _returnvalue
            (set `self.LockOnTarget` (`.HitActor` (`GameplayStatics.BreakHitResult` _outhit)))))))))

(event `fireEffectServer`
  ;[0.7157 1 0.8148] Apply Damage & Die
  (`self.fireEffectMulticast`))

(event `self.ReceiveAnyDamage`
  (params (Damage :type "Float (single-precision)") (DamageType :type "DamageType Object Reference") (InstigatedBy :type "Controller Object Reference") (DamageCauser :type "Actor Object Reference"))
  (bind _returnvalue (`GameplayStatics.GetObjectClass` DamageType))
  ;[0.7157 1 0.8148] Apply Damage & Die
  (if (== _returnvalue "/Game/2_BP/DamageType/DT_Fire.DT_Fire_C")
    (if (not (`self.noDamageTime`))
      (`KismetSystemLibrary.PrintString` "fire!!!!!!!" false)
      (set `self.State_HP` (- (`self.State_HP`) Damage))
      (set `self.noDamageTime` true)
      (`KismetSystemLibrary.Delay` 0.5)
      (set `self.noDamageTime` false))
    (elif (== _returnvalue "/Game/2_BP/DamageType/DT_Laser.DT_Laser_C")
      (`KismetSystemLibrary.PrintString` "tailATK hit!!!" false :!label _label)
      (if (`self.bIsNoHit`)
        (set `self.State_HP` (- (`self.State_HP`) Damage))
        (`self.playHitSound`)
        (set `self.bIsNoHit` false)
        (`self.hitEffectServer`))
      (elif (== _returnvalue "/Game/2_BP/DamageType/DT_Ice.DT_Ice_C")
        (if (`self.noDamageTime`)
          _
          (elif (`self.bIsNoHit`)
            (`KismetSystemLibrary.PrintString` "cold!!!!!" false)
            (set `self.State_HP` (- (`self.State_HP`) Damage))
            (set `self.bIsNoHit` false)
            (set `self.noDamageTime` true)
            (set `CharacterMovementComponent.MaxWalkSpeed` (* 50.0 (`self.SpeedStat`)) (`self.CharacterMovement`))
            (`KismetSystemLibrary.Delay` 0.5)
            (set `self.bIsNoHit` true)
            (`KismetSystemLibrary.Delay` 5.0)
            (set `self.noDamageTime` false)
            (set `CharacterMovementComponent.MaxWalkSpeed` (* 150.0 (`self.SpeedStat`)) (`self.CharacterMovement`))))
        (elif (== _returnvalue "/Game/2_BP/DamageType/DT_Tail.DT_Tail_C")
          (goto _label)
          (elif (== _returnvalue "/Game/2_BP/DamageType/DT_Bite.DT_Bite_C")
            (goto _label)
            (elif (== _returnvalue "/Game/2_BP/DamageType/DT_Roar.DT_Roar_C")
              (goto _label))))))))

(event `fireEffectMulticast`
  ;[0.7157 1 0.8148] Apply Damage & Die
  (`GameplayStatics.SpawnEmitterAttached` "/Game/StarterContent/Particles/P_Fire.P_Fire" (`self.CapsuleComponent`) "None" (0.0 110.0 0.0)))

(event `self.ReceiveTick`
  (params (DeltaSeconds :type "Float (single-precision)"))
  (bind _returnvalue (`self.GetController`))
  ;[0.1489 0.2268 0.3438] Lock On System
  (`self.LockOnTarget`
    (:`then`
      (`/Engine/EditorBlueprintResources/StandardMacros.IsValid` _returnvalue
        (:`Is Valid`
          (`Controller.SetControlRotation` _returnvalue (`KismetMathLibrary.FindLookAtRotation` (`self.K2_GetActorLocation`) (`self.K2_GetActorLocation` (`self.LockOnTarget`))))
          (`KismetSystemLibrary.PrintString` (`KismetStringLibrary.Conv_DoubleToString` (`SpringArmComponent.TargetArmLength` (`self.PlayerCamArm`))) true true (struct :`G` 0.66 :`B` 1.0 :`A` 1.0) DeltaSeconds))))
    (:`else`)))

(event `EnhancedInput|/Game/7_MISC/Input/IA_PlayerLook`
  (params (ActionValue :type "Vector2D Structure") (ElapsedSeconds :type "Float (double-precision)") (TriggeredSeconds :type "Float (double-precision)") (InputAction :type "InputAction Object Reference" :default "/Game/7_MISC/Input/IA_PlayerLook.IA_PlayerLook"))
  ;[0.1665 0.08562 0.2292] In Place Turn
  (:`Triggered`
    (if (== (`KismetMathLibrary.VSize` (`MovementComponent.Velocity` (`self.CharacterMovement`))) 0.0)
      (`|ExecutionSequence`
        (:`then_0`
          (if (>= ActionValue_X 0.7)
            (set `self.bTurnRight` true)
            (set `self.bTurnLeft` false)
            (else
              (set `self.bTurnRight` false))))
        (:`then_1`
          (if (<= ActionValue_X -0.7)
            (set `self.bTurnLeft` true)
            (set `self.bTurnRight` false)
            (else
              (set `self.bTurnLeft` false)))))
      (else
        (set `self.bTurnLeft` false)
        (set `self.bTurnRight` false)))))

(event `hitEffectServer`
  ;[0.7186 1 0.8171] Comment
  (`self.hitEffectMulticast`))

(event `hitZoomIn`
  ;[0.7157 1 0.8148] Hit Zoom In
  (bind (_direction _sprinarmlength) (`Timeline|Timeline_5` :!via `PlayFromStart`)
    (:`Update`
      (set `SpringArmComponent.TargetArmLength` _sprinarmlength (`self.PlayerCamArm`)))
    (:`Finished`
      (bind (_direction_2 _sprinarmlength_2) (`Timeline|Timeline_6` :!via `ReverseFromEnd`)
        (:`Update`
          (set `SpringArmComponent.TargetArmLength` _sprinarmlength_2 (`self.PlayerCamArm`)))))))

(event `hitEffectMulticast`
  ;[0.7186 1 0.8171] Comment
  (if (<= (`self.State_HP`) 0.0)
    ;;[0 0.06098 1] Die
    (`GameplayStatics.PlayWorldCameraShake` "/Game/2_BP/CameraShaking/BP_GetHit.BP_GetHit_C" (`self.K2_GetActorLocation`) 0.0 2000.0)
    (`SkeletalMeshComponent.PlayAnimation` (`self.Mesh`) "/Game/7_MISC/Animation/BlueTRex/BS/BlueTRex_A_012_TRexSue_Die_Anim.BlueTRex_A_012_TRexSue_Die_Anim" false)
    (set `CharacterMovementComponent.MaxWalkSpeed` 0.0 (`self.CharacterMovement`))
    (else
      ;;[1 0.304 0.6201] Damage
      (set `CharacterMovementComponent.MaxWalkSpeed` 0.0 (`self.CharacterMovement`))
      (set `self.bUseControllerRotationYaw` false)
      (`KismetSystemLibrary.Delay` 1.0)
      (set `self.bIsNoHit` true))))

(event `EnhancedInput|/Game/7_MISC/Input/IA_Basic_TailAttack`
  (params (ActionValue :type Boolean) (ElapsedSeconds :type "Float (double-precision)") (TriggeredSeconds :type "Float (double-precision)") (InputAction :type "InputAction Object Reference" :default "/Game/7_MISC/Input/IA_Basic_TailAttack.IA_Basic_TailAttack"))
  ;[0.03646 0.03646 0.03646] Basic Attack
  ;;[1 0 0] TailAttack
  (:`Started`
    (`self.TailAttack_Server`)))

(event `TailAttack_Server`
  ;[0.03646 0.03646 0.03646] Basic Attack
  ;;[1 0 0] TailAttack
  (`self.TailAttack_Multicast`))

(event `flameProjectileSpawner`
  ;[0.03689 0.03689 0.03689] Special Skill
  ;;[1 0.5647 0.3005] 화염방사 충돌체 생성
  (if (`self.bFlameOnOff`) :!label _label_2
    (`|SpawnActorFromClass` "/Game/2_BP/BP_FlameProjectile.BP_FlameProjectile_C" (`KismetMathLibrary.MakeTransform` (`SceneComponent.GetSocketLocation` (`self.PlayerBody`) "bn_Jaw_11") (struct) (10.0 10.0 10.0)) "AlwaysSpawn" "MultiplyWithRoot" self null)
    (`KismetSystemLibrary.Delay` 0.2)
    (goto _label_2)))

(event `TailAttack_Multicast`
  ;[0.03646 0.03646 0.03646] Basic Attack
  ;;[1 0 0] TailAttack
  (if (not (`self.bTailAttack`))
    (set `self.bTailAttack` true)
    (set `CharacterMovementComponent.MaxWalkSpeed` 0.0 (`self.CharacterMovement`))
    (set `self.bUseControllerRotationYaw` false)
    (`self.DisableInput` null)))

(event `EnhancedInput|/Game/7_MISC/Input/IA_SpecialSkill`
  (params (ActionValue :type Boolean) (ElapsedSeconds :type "Float (double-precision)") (TriggeredSeconds :type "Float (double-precision)") (InputAction :type "InputAction Object Reference" :default "/Game/7_MISC/Input/IA_SpecialSkill.IA_SpecialSkill"))
  ;[0.03689 0.03689 0.03689] Special Skill
  (:`Started`
    (`self.flameThrowerServer`)))

(event `TailAttack_End`
  ;[0.03646 0.03646 0.03646] Basic Attack
  ;;[1 0 0] TailAttack
  (if (`self.bTailAttack`)
    (set `self.bTailAttack` false)
    (set `CharacterMovementComponent.MaxWalkSpeed` 600.0 (`self.CharacterMovement`))
    (set `self.bUseControllerRotationYaw` true)
    (`self.EnableInput` null)))

(event `flameThrowerServer`
  ;[0.03689 0.03689 0.03689] Special Skill
  (`self.flameThrowerMulticast`))

(event `EnhancedInput|/Game/7_MISC/Input/IA_Basic_Bite`
  (params (ActionValue :type Boolean) (ElapsedSeconds :type "Float (double-precision)") (TriggeredSeconds :type "Float (double-precision)") (InputAction :type "InputAction Object Reference" :default "/Game/7_MISC/Input/IA_Basic_Bite.IA_Basic_Bite"))
  ;[0.03646 0.03646 0.03646] Basic Attack
  ;;[1 0 0.1714] Bite
  (:`Started`
    (`self.BiteAttack_Server`)))

(event `flameThrowerMulticast`
  (bind _iceattacklocvector (`self.iceAttackLocVector`))
  (bind _charactermovement (`self.CharacterMovement`))
  (bind (_returnvalue_roll _returnvalue_pitch _returnvalue_yaw) (`KismetMathLibrary.BreakRotator` (`KismetMathLibrary.Conv_VectorToRotator` (`self.GetActorForwardVector`))))
  (bind (_returnvalue_roll_2 _returnvalue_pitch_2 _returnvalue_yaw_2) (`KismetMathLibrary.BreakRotator` (`KismetMathLibrary.Conv_VectorToRotator` (`self.GetActorForwardVector`))))
  ;[0.03689 0.03689 0.03689] Special Skill
  (if (`self.CoolTime_SpecialSkill`)
    (`KismetSystemLibrary.PrintString` "coolTime!!!!" false true (struct :`R` 1.0 :`G` 0.960876 :`A` 1.0))
    (else
      (set `self.CoolTime_SpecialSkill` false)
      (switch `int` (`self.SpecialSkill`)
        (:`Default`
          ;;[1 0.5647 0.3005] 화염방사 스킬
          (`|ExecutionSequence` :!label _label_3
            (:`then_0`
              (`|PlayMontage` (`self.PlayerBody`) "/Game/7_MISC/Animation/BlueTRex/Skill/FireBreath/BlueTRex_014_ck2_Anim_FireBreath_Montage3.BlueTRex_014_ck2_Anim_FireBreath_Montage3" 1.0 0.0 "None"
                (:`then`
                  (bind (_direction _firebreathaim) (`Timeline|Timeline_4` :!label _label_4)
                    (:`Update`
                      (set `SpringArmComponent.TargetArmLength` (`KismetMathLibrary.Lerp` 600.0 350.0 _firebreathaim) (`self.PlayerCamArm`)))))
                (:`OnCompleted`
                  (goto _label_4 :!via `Reverse`))))
            (:`then_1`
              (`ActorComponent.ToggleActive` (`self.Skill Nia Effect`))
              (set `self.bFlameOnOff` true)
              (`self.flameProjectileSpawner`)
              (`KismetSystemLibrary.Delay` 5.0)
              (`ActorComponent.Deactivate` (`self.Skill Nia Effect`))
              (set `self.bFlameOnOff` false)
              (`KismetSystemLibrary.Delay` 5.0)
              (set `self.CoolTime_SpecialSkill` false)
              (`KismetSystemLibrary.PrintString` "coolDown!!!!!!" false :!label _label_5))))
        (:`0`
          (goto _label_3))
        (:`1`
          ;;[0.2462 1 0.9216] Notify_LaserBeam_Start
          (if (not (`self.bLaserBeam`))
            (set `self.bLaserBeam` true)
            (set `CharacterMovementComponent.MaxWalkSpeed` 0.0 (`self.CharacterMovement`))
            (set `self.bUseControllerRotationYaw` false)))
        (:`2`
          ;;[0.3265 0.6439 1] 얼음 스킬
          (`|PlayMontage` (`self.PlayerBody`) "/Game/7_MISC/Animation/BlueTRex/Skill/ICEStalagmite/BlueTRex_IceStalagmite_Montage.BlueTRex_IceStalagmite_Montage"
            (:`then`
              (set `self.bICEStalagmite` true)
              (set `CharacterMovementComponent.MaxWalkSpeed` 0.0 _charactermovement))
            (:`OnCompleted`
              (set `self.bICEStalagmite` false)
              (set `CharacterMovementComponent.MaxWalkSpeed` 600.0 _charactermovement))
            (:`OnNotifyBegin`
              (`ActorComponent.ToggleActive` (`self.Skill Emitter Effect 2`))
              (`SceneComponent.K2_SetWorldLocation` (`self.Skill Emitter Effect 2`) (`SceneComponent.GetSocketLocation` (`self.PlayerBody`) "bn_RightFootMiddle2_63") false false)
              (`SceneComponent.K2_SetWorldRotation` (`self.Skill Emitter Effect 2`) (`KismetMathLibrary.MakeRotator` _returnvalue_roll _returnvalue_pitch (+ _returnvalue_yaw -90.0)) false false)
              (`KismetSystemLibrary.Delay` 0.2)
              (`ActorComponent.ToggleActive` (`self.Skill Emitter Effect`))
              (`SceneComponent.K2_SetWorldLocation` (`self.Skill Emitter Effect`) (`SceneComponent.GetSocketLocation` (`self.PlayerBody`) "bn_RightFootMiddle2_63") false false)
              (`SceneComponent.K2_SetWorldRotation` (`self.Skill Emitter Effect`) (`KismetMathLibrary.MakeRotator` _returnvalue_roll_2 _returnvalue_pitch_2 (+ _returnvalue_yaw_2 -90.0)) false false)
              (set `self.iceAttackFwdVector` (`self.GetActorForwardVector`))
              (set `self.iceAttackLocVector` (`SceneComponent.GetSocketLocation` (`self.PlayerBody`) "bn_RightFootMiddle2_63"))
              (bind (_direction_2 _newtrack_1) (`Timeline|Timeline_3` :!via `PlayFromStart`)
                (:`Update`
                  (for _index (range 3)
                    (bind (_outhit _returnvalue) (`KismetSystemLibrary.BoxTraceSingleForObjects` :`Start` _iceattacklocvector :`End` (+ _iceattacklocvector (* (`KismetMathLibrary.GreaterGreater_VectorRotator` (`self.iceAttackFwdVector`) (`KismetMathLibrary.MakeRotator` 0.0 0.0 (`KismetMathLibrary.Conv_IntToDouble` (- (* _index 20) 20)))) (* _newtrack_1 1000.0))) :`HalfSize` (50.0 50.0 50.0) :`ObjectTypes` (`|MakeArray` "ObjectTypeQuery3" :!type "EObjectTypeQuery Enum") :`DrawDebugType` "ForOneFrame" :`DrawTime` (`self.GetActorTickInterval`)))
                    (if _returnvalue
                      (`GameplayStatics.ApplyDamage` (`.HitActor` (`GameplayStatics.BreakHitResult` _outhit)) (* (`self.PowerStat`) 1.0) null null "/Game/2_BP/DamageType/DT_Ice.DT_Ice_C")
                      (`self.HitMarkerMaker`)
                      (`KismetSystemLibrary.PrintString` "coolDown!!!!!!" false))))
                (:`Finished`
                  (`KismetSystemLibrary.Delay` 5.0)
                  (set `self.CoolTime_SpecialSkill` false))))))))))

(event `BiteAttack_Server`
  ;[0.03646 0.03646 0.03646] Basic Attack
  ;;[1 0 0.1714] Bite
  (`self.BiteAttack_Multicast`))

(event `BiteAttack_Multicast`
  ;[0.03646 0.03646 0.03646] Basic Attack
  ;;[1 0 0.1714] Bite
  (if (not (`self.bBite`))
    (set `self.bBite` true)
    (`|PlayMontage` (`self.PlayerBody`) "/Game/7_MISC/Animation/BlueTRex/Skill/Bite/BlueTRex_Attack_biteShaking_2_Montage.BlueTRex_Attack_biteShaking_2_Montage"
      (:`OnCompleted`
        (set `self.bBite` false)))))

(event `EnhancedInput|/Game/7_MISC/Input/IA_Basic_Roar`
  (params (ActionValue :type Boolean) (ElapsedSeconds :type "Float (double-precision)") (TriggeredSeconds :type "Float (double-precision)") (InputAction :type "InputAction Object Reference" :default "/Game/7_MISC/Input/IA_Basic_Roar.IA_Basic_Roar"))
  ;[0.03646 0.03646 0.03646] Basic Attack
  ;;[1 0.4233 0] Roar
  (:`Started`
    (`self.RoarAttack_Server`)))

(event `LaserBeam_Start`
  ;[0.03689 0.03689 0.03689] Special Skill
  ;;[0.2462 1 0.9216] Notify_LaserBeam_Start
  (`self.LaserBeam_Start_Multicast`))

(event `LaserBeam_Start_Multicast`
  (bind _playerbody (`self.PlayerBody`))
  (bind _returnvalue (`SceneComponent.GetSocketLocation` _playerbody "bn_Tongue3_14"))
  ;[0.03689 0.03689 0.03689] Special Skill
  ;;[0.2462 1 0.9216] Notify_LaserBeam_Start
  ;;[0.2462 1 0.9216] 레이저 스킬
  (`ActorComponent.ToggleActive` (`self.Skill Nia Effect`))
  (bind (_outhit _returnvalue_2) (`KismetSystemLibrary.SphereTraceSingleForObjects` :`Start` _returnvalue :`End` (+ _returnvalue (* (`SceneComponent.GetRightVector` _playerbody) 800.0)) :`Radius` 20.0 :`ObjectTypes` (`|MakeArray` "ObjectTypeQuery3" "ObjectTypeQuery9" "ObjectTypeQuery10" :!type "EObjectTypeQuery Enum") :`DrawDebugType` "ForDuration"))
  (`|ExecutionSequence`
    (:`then_0`
      (if _returnvalue_2
        (`GameplayStatics.ApplyDamage` (`.HitActor` (`GameplayStatics.BreakHitResult` _outhit)) (* (`self.PowerStat`) 5.0) null null "/Game/2_BP/DamageType/DT_Laser.DT_Laser_C")
        (`self.HitMarkerMaker`)))
    (:`then_1`
      (`KismetSystemLibrary.Delay` 5.0)
      (set `self.CoolTime_SpecialSkill` false)
      (goto _label_5))))

(event `RoarAttack_Server`
  ;[0.03646 0.03646 0.03646] Basic Attack
  ;;[1 0.4233 0] Roar
  (`self.RoarAttack_Multicast`))

(event `RoarAttack_Multicast`
  ;[0.03646 0.03646 0.03646] Basic Attack
  ;;[1 0.4233 0] Roar
  (set `self.bRoar` true)
  (set `CharacterMovementComponent.MaxWalkSpeed` 0.0 (`self.CharacterMovement`))
  (set `self.bUseControllerRotationYaw` false))

(event `RoarAttack_End`
  ;[0.03646 0.03646 0.03646] Basic Attack
  ;;[1 0.4233 0] Roar
  (`self.RoarAttack_End_Multicast`))

(event `RoarAttack_End_Multicast`
  ;[0.03646 0.03646 0.03646] Basic Attack
  ;;[1 0.4233 0] Roar
  (set `self.bRoar` false)
  (set `CharacterMovementComponent.MaxWalkSpeed` 600.0 (`self.CharacterMovement`))
  (set `self.bUseControllerRotationYaw` true))

(event `LaserBeam_End`
  ;[0.03689 0.03689 0.03689] Special Skill
  ;;[0.2462 1 0.9216] Notify_LaserBeam_End
  (`self.LaserBeam_End_Multicast`))

(event `LaserBeam_End_Multicast`
  ;[0.03689 0.03689 0.03689] Special Skill
  ;;[0.2462 1 0.9216] Notify_LaserBeam_End
  (set `self.bLaserBeam` false)
  (set `CharacterMovementComponent.MaxWalkSpeed` (* 150.0 (`self.SpeedStat`)) (`self.CharacterMovement`))
  (set `self.bUseControllerRotationYaw` true))

(event `BuffSkillMulticast`
  (bind _tempstat (`self.TempStat`))
  ;[1 0.8963 0.3185] buff Skill
  (if (`self.CoolTime_BuffSkill`)
    (`KismetSystemLibrary.PrintString` "buff cool time !!!!!" false)
    (else
      (set `self.CoolTime_BuffSkill` false)
      (switch `int` (`self.BuffSkill`)
        (:`0`
          (bind _output_get (set `self.TempStat` (`self.PowerStat`)))
          (set `self.TempStat` (+ _output_get 3.0))
          (`ActorComponent.SetActive` (`self.Buff Effect`) true false :!label _label_6)
          (`KismetSystemLibrary.Delay` 6.0)
          (switch `int` (`self.BuffSkill`)
            (:`0`
              (set `self.PowerStat` _tempstat))
            (:`1`
              (set `self.DefenceStat` _tempstat))
            (:`2`
              (set `self.SpeedStat` _tempstat)
              (set `CharacterMovementComponent.MaxWalkSpeed` (* 150.0 (`self.SpeedStat`)) (`self.CharacterMovement`))))
          (`ActorComponent.SetActive` (`self.Buff Effect`) false false)
          (`KismetSystemLibrary.Delay` 10.0)
          (set `self.CoolTime_BuffSkill` false))
        (:`1`
          (bind _output_get_2 (set `self.TempStat` (`self.DefenceStat`)))
          (set `self.TempStat` 0.0))
        (:`2`
          (bind _output_get_3 (set `self.TempStat` (`self.SpeedStat`)))
          (set `self.SpeedStat` (+ _output_get_3 3.0))
          (set `CharacterMovementComponent.MaxWalkSpeed` (* 150.0 (`self.SpeedStat`)) (`self.CharacterMovement`))
          (goto _label_6))))))

(event `EnhancedInput|/Game/7_MISC/Input/IA_BuffSkill`
  (params (ActionValue :type Boolean) (ElapsedSeconds :type "Float (double-precision)") (TriggeredSeconds :type "Float (double-precision)") (InputAction :type "InputAction Object Reference" :default "/Game/7_MISC/Input/IA_BuffSkill.IA_BuffSkill"))
  ;[1 0.8963 0.3185] buff Skill
  (:`Started`
    (`self.BuffSkillServer`)))

(event `BuffSkillServer`
  ;[1 0.8963 0.3185] buff Skill
  (`self.BuffSkillMulticast`))

(fn `buffSkillEffectMaker`
  (switch `int` (`self.BuffSkill`)
    (:`Default`
      (bind _returnvalue (`NiagaraFunctionLibrary.SpawnSystemAttached` "/Game/5_FX/NS_PowerBuffEffect.NS_PowerBuffEffect" (`self.CapsuleComponent`) "None" (0.0 -0.0 -88.0) (struct :`Yaw` 90.0) "KeepRelativeOffset" false false :!label _label))
      (set `self.Buff Effect` _returnvalue))
    (:`0`
      (goto _label))
    (:`1`
      (bind _returnvalue_2 (`NiagaraFunctionLibrary.SpawnSystemAttached` "/Game/5_FX/NS_HealBuffEffect.NS_HealBuffEffect" (`self.CapsuleComponent`) "None" (0.0 -0.0 -88.0) (struct) "KeepRelativeOffset" false false))
      (set `self.Buff Effect` _returnvalue_2))
    (:`2`
      (bind _returnvalue_3 (`NiagaraFunctionLibrary.SpawnSystemAttached` "/Game/5_FX/NS_SpeedBuffEffect.NS_SpeedBuffEffect" (`self.CapsuleComponent`) "None" (0.0 -0.0 -88.0) (struct) "KeepRelativeOffset" false false))
      (set `self.Buff Effect` _returnvalue_3))))

(fn `HitMarkerMaker`
  (`self.hitZoomIn`)
  (`KismetSystemLibrary.PrintString` "Hello"))

(fn `playHitSound`
  (locals (sound2Play :type "SoundBase Object Reference"))
  (switch `int` (`KismetMathLibrary.RandomIntegerInRange` 0 2)
    (:`0`
      (set `local.sound2Play` "/Game/8_SOUND/DinoHitSound/Smash_Hit_Sound_Effects_HD__mp3cut_net_.Smash_Hit_Sound_Effects_HD__mp3cut_net_"))
    (:`1`
      (set `local.sound2Play` "/Game/8_SOUND/DinoHitSound/Smash_Hit_Sound_Effects_HD__mp3cut_net___1_.Smash_Hit_Sound_Effects_HD__mp3cut_net___1_"))
    (:`2`
      (set `local.sound2Play` "/Game/8_SOUND/DinoHitSound/Smash_Hit_Sound_Effects_HD__mp3cut_net___2_.Smash_Hit_Sound_Effects_HD__mp3cut_net___2_")))
  (`GameplayStatics.PlaySoundAtLocation` (`local.sound2Play`) (`self.K2_GetActorLocation`) (struct) 1.0 1.0 0.0 "/Game/8_SOUND/PlayerSoundAttenuation.PlayerSoundAttenuation" null null null))

(fn `SpecialSkillEffectMaker`
  (switch `int` (`self.SpecialSkill`)
    (:`0`
      (bind _returnvalue (`NiagaraFunctionLibrary.SpawnSystemAttached` "/Game/DragonFlameFX/FX/NS_DragonFlame_Fire1.NS_DragonFlame_Fire1" (`self.PlayerBody`) "bn_Jaw_11" (0.0 0.0 0.0) (struct :`Pitch` -20.0) "KeepRelativeOffset" false false))
      (set `self.Skill Nia Effect` _returnvalue))
    (:`1`
      (bind _returnvalue_2 (`NiagaraFunctionLibrary.SpawnSystemAttached` "/Game/5_FX/VFX_Laser1.VFX_Laser1" (`self.PlayerBody`) "LaserBeam_Point" (0.0 0.0 0.0) (`KismetMathLibrary.Conv_VectorToRotator` (* (`self.GetActorForwardVector`) (-1.0 0.0 0.0))) "KeepRelativeOffset" false false))
      (set `self.Skill Nia Effect` _returnvalue_2))
    (:`2`
      (bind _returnvalue_3 (`GameplayStatics.SpawnEmitterAtLocation` "/Game/5_FX/P_IceGroundAttack17.P_IceGroundAttack17" (0.0 0.0 0.0) (struct) (1.0 1.5 1.5) false "None" false))
      (set `self.Skill Emitter Effect` _returnvalue_3)
      (bind _returnvalue_4 (`GameplayStatics.SpawnEmitterAtLocation` "/Game/5_FX/P_IceGroundAttack171.P_IceGroundAttack171" (0.0 0.0 0.0) (struct) (1.0 0.5 0.5) false "None" false))
      (set `self.Skill Emitter Effect 2` _returnvalue_4))))

(fn `UserConstructionScript`
  (bind _playerbody (`self.PlayerBody`))
  (`SceneComponent.K2_AttachToComponent` (`self.PlayerTailCollision`) _playerbody "bn_Tail05_71" "KeepRelative" "KeepRelative" "KeepRelative" true)
  (`SceneComponent.K2_AttachToComponent` (`self.PlayerUpperBodyCollision`) _playerbody "bn_Neck_7" "KeepRelative" "KeepRelative" "KeepRelative" true)
  (`SceneComponent.K2_AttachToComponent` (`self.PlayerHeadCollision`) _playerbody "bn_Head_10" "KeepRelative" "KeepRelative" "KeepRelative" true)
  (`SceneComponent.K2_AttachToComponent` (`self.HP_Bar`) _playerbody "HP_Bar" "KeepRelative" "KeepRelative" "KeepRelative" true))