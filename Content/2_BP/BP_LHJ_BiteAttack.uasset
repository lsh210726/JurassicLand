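; Anim notify state that applies bite damage for BP_BlueTRex during an attack animation.
; Each tick it sphere-traces between the tongue and upper jaw sockets against pawns and two other object types.
; A hit deals DT_Bite damage scaled by PowerStat, triggers the hit marker, spawns blood and knocks Characters back along the impact normal.
; No already-hit guard exists, so damage can repeat every tick.
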(fn `Received_NotifyTick`
  (params (MeshComp :type "SkeletalMeshComponent Object Reference") (Animation :type "AnimSequenceBase Object Reference") (FrameDeltaTime :type "Float (single-precision)") (EventReference :type "AnimNotifyEventReference Structure (by ref)"))
  (returns (ReturnValue :type Boolean))
  (bind (_outhit _returnvalue) (`KismetSystemLibrary.SphereTraceSingleForObjects` MeshComp (`SceneComponent.GetSocketLocation` MeshComp "bn_Tongue1_12") (`SceneComponent.GetSocketLocation` MeshComp "Upper_Jaw") 80.0 (`|MakeArray` "ObjectTypeQuery3" "ObjectTypeQuery9" "ObjectTypeQuery10" :!type "EObjectTypeQuery Enum")))
  (if _returnvalue
    (bind _asbp_blue_trex (cast `/Game/2_BP/BP_BlueTRex` (`ActorComponent.GetOwner` MeshComp)))
    (bind (_bblockinghit _binitialoverlap _time _distance _location _impactpoint _normal _impactnormal _physmat _hitactor) (`GameplayStatics.BreakHitResult` _outhit))
    (`GameplayStatics.ApplyDamage` _hitactor (* (`/Game/2_BP/BP_BlueTRex.powerStat` _asbp_blue_trex) 2.0) null null "/Game/2_BP/DamageType/DT_Bite.DT_Bite_C")
    (`/Game/2_BP/BP_BlueTRex.HitMarkerMaker` _asbp_blue_trex)
    (`GameplayStatics.SpawnEmitterAtLocation` _hitactor "/Game/Realistic_Starter_VFX_Pack_Vol2/Particles/Blood/P_Blood_Splat_Cone.P_Blood_Splat_Cone" _impactpoint (`KismetMathLibrary.MakeRotFromZ` _normal) (2.0 2.0 2.0))
    (bind _ascharacter (cast `Character` _hitactor))
    (bind (_returnvalue_x _returnvalue_y) (`KismetMathLibrary.BreakVector` (* _normal -300.0)))
    (`Character.LaunchCharacter` _ascharacter (`KismetMathLibrary.MakeVector` _returnvalue_x _returnvalue_y 10.0) false false)
    (return false)))