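; BP_InvisibleWall is an actor that gathers BP_BlueTRex actors as players and updates its own transform, presumably to act as an invisible barrier.
; Three seconds after BeginPlay it caches those actors in Players.
; Each Tick computes their average location without using it, then sets location and rotation with no location supplied and a look-at from its own location to itself, so it does not track the players.
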(event `self.ReceiveBeginPlay`
  (`KismetSystemLibrary.Delay` 3.0)
  (bind _outactors (`GameplayStatics.GetAllActorsOfClass` "/Game/2_BP/BP_BlueTRex.BP_BlueTRex_C"))
  (bind _output_get (set `self.players` _outactors)))

(event `self.ReceiveTick`
  (params (DeltaSeconds :type "Float (single-precision)"))
  (`GameplayStatics.GetActorArrayAverageLocation` (`self.players`))
  (`self.K2_SetActorLocationAndRotation` (0.0 0.0 0.0) (`KismetMathLibrary.FindLookAtRotation` (`self.K2_GetActorLocation`) (`self.K2_GetActorLocation`))))

(fn `UserConstructionScript`)