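; Anim notify state for the Raptor's roar attack, dealing area damage in front of the mesh while the notify is active.
; Each tick sphere-traces along the mesh's right vector for pawns and two custom object types.
; A hit triggers a world camera shake at the Raptor, applies roar damage scaled from its PowerStat and spawns blood at the impact.
; Hit Characters are also launched against the impact normal with a slight lift.
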(fn `Received_NotifyTick`
  (params (MeshComp :type "SkeletalMeshComponent Object Reference") (Animation :type "AnimSequenceBase Object Reference") (FrameDeltaTime :type "Float (single-precision)") (EventReference :type "AnimNotifyEventReference Structure (by ref)"))
  (returns (ReturnValue :type Boolean))
  (bind _returnvalue (`ActorComponent.GetOwner` MeshComp))
  (bind _ascharacter (cast `Character` _returnvalue))
  (bind _mesh (`Character.Mesh` _ascharacter))
  (bind _returnvalue_2 (`SceneComponent.K2_GetComponentLocation` _mesh))
  (bind (_outhit _returnvalue_3) (`KismetSystemLibrary.SphereTraceSingleForObjects` MeshComp _returnvalue_2 (+ _returnvalue_2 (* (`KismetMathLibrary.GetRightVector` (`SceneComponent.K2_GetComponentRotation` _mesh)) 500.0)) 300.0 (`|MakeArray` "ObjectTypeQuery3" "ObjectTypeQuery9" "ObjectTypeQuery10" :!type "EObjectTypeQuery Enum")))
  (if _returnvalue_3
    (bind _asraptor (cast `Raptor` _returnvalue))
    (`GameplayStatics.PlayWorldCameraShake` _asraptor "/Game/2_BP/CameraShaking/BP_Roar_CamShake.BP_Roar_CamShake_C" (`Actor.K2_GetActorLocation` _asraptor) 0.0 1000.0)
    (bind (_bblockinghit _binitialoverlap _time _distance _location _impactpoint _normal _impactnormal _physmat _hitactor) (`GameplayStatics.BreakHitResult` _outhit))
    (`GameplayStatics.ApplyDamage` _hitactor (* (`BasePlayer.PowerStat` _asraptor) 0.5) null null "/Game/2_BP/DamageType/DT_Roar.DT_Roar_C")
    (`GameplayStatics.SpawnEmitterAtLocation` _hitactor "/Game/Realistic_Starter_VFX_Pack_Vol2/Particles/Blood/P_Blood_Splat_Cone.P_Blood_Splat_Cone" _impactpoint (`KismetMathLibrary.MakeRotFromZ` _normal) (2.0 2.0 2.0))
    (bind _ascharacter_2 (cast `Character` _hitactor))
    (bind (_returnvalue_x _returnvalue_y) (`KismetMathLibrary.BreakVector` (* _normal -70.0)))
    (`Character.LaunchCharacter` _ascharacter_2 (`KismetMathLibrary.MakeVector` _returnvalue_x _returnvalue_y 10.0) false false)
    (return false)))