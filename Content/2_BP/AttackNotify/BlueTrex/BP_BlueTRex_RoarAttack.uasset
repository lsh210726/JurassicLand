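; Anim notify state for BlueTRex's roar attack, which damages and knocks characters during the animation window.
; On begin, it plays the roar sound and Niagara impact effect at the LaserBeam_Point socket.
; Each tick sphere-traces along the mesh's right vector.
; Every tick with a hit plays a camera shake, applies damage scaled from PowerStat, spawns blood and launches hit characters along the negated hit normal, so damage can repeat.
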(fn `Received_NotifyBegin`
  (params (MeshComp :type "SkeletalMeshComponent Object Reference") (Animation :type "AnimSequenceBase Object Reference") (TotalDuration :type "Float (single-precision)") (EventReference :type "AnimNotifyEventReference Structure (by ref)"))
  (returns (ReturnValue :type Boolean))
  (bind _returnvalue (`SceneComponent.GetSocketLocation` MeshComp "LaserBeam_Point"))
  (`GameplayStatics.PlaySoundAtLocation` MeshComp "/Game/8_SOUND/roarsound3.roarsound3" _returnvalue (struct) 1.0 1.0 0.0 "/Game/8_SOUND/PlayerSoundAttenuation.PlayerSoundAttenuation" null null null)
  (`NiagaraFunctionLibrary.SpawnSystemAtLocation` MeshComp "/Game/Realistic_Starter_VFX_Pack_Niagara/Niagara/Explosion/NS_RoarImpact.NS_RoarImpact" _returnvalue)
  (return false))

(fn `Received_NotifyTick`
  (params (MeshComp :type "SkeletalMeshComponent Object Reference") (Animation :type "AnimSequenceBase Object Reference") (FrameDeltaTime :type "Float (single-precision)") (EventReference :type "AnimNotifyEventReference Structure (by ref)"))
  (returns (ReturnValue :type Boolean))
  (bind _returnvalue (`ActorComponent.GetOwner` MeshComp))
  (bind _ascharacter (cast `Character` _returnvalue))
  (bind _mesh (`Character.Mesh` _ascharacter))
  (bind _returnvalue_2 (`SceneComponent.K2_GetComponentLocation` _mesh))
  (bind (_outhit _returnvalue_3) (`KismetSystemLibrary.SphereTraceSingleForObjects` MeshComp _returnvalue_2 (+ _returnvalue_2 (* (`KismetMathLibrary.GetRightVector` (`SceneComponent.K2_GetComponentRotation` _mesh)) 500.0)) 300.0 (`|MakeArray` "ObjectTypeQuery3" "ObjectTypeQuery9" "ObjectTypeQuery10" :!type "EObjectTypeQuery Enum")))
  (if _returnvalue_3
    (bind _asbp_blue_trex (cast `/Game/2_BP/BP_BlueTRex` _returnvalue))
    (`GameplayStatics.PlayWorldCameraShake` _asbp_blue_trex "/Game/2_BP/CameraShaking/BP_Roar_CamShake.BP_Roar_CamShake_C" (`Actor.K2_GetActorLocation` _asbp_blue_trex) 0.0 1000.0)
    (bind (_bblockinghit _binitialoverlap _time _distance _location _impactpoint _normal _impactnormal _physmat _hitactor) (`GameplayStatics.BreakHitResult` _outhit))
    (`GameplayStatics.ApplyDamage` _hitactor (* (`/Game/2_BP/BP_BlueTRex.powerStat` _asbp_blue_trex) 0.5))
    (`GameplayStatics.SpawnEmitterAtLocation` _hitactor "/Game/Realistic_Starter_VFX_Pack_Vol2/Particles/Blood/P_Blood_Splat_Cone.P_Blood_Splat_Cone" _impactpoint (`KismetMathLibrary.MakeRotFromZ` _normal) (2.0 2.0 2.0))
    (bind _ascharacter_2 (cast `Character` _hitactor))
    (bind (_returnvalue_x _returnvalue_y) (`KismetMathLibrary.BreakVector` (* _normal -70.0)))
    (`Character.LaunchCharacter` _ascharacter_2 (`KismetMathLibrary.MakeVector` _returnvalue_x _returnvalue_y 10.0) false false)
    (return false)))