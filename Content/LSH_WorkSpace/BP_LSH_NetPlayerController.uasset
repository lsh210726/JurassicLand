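; BP_LSH_NetPlayerController is a network player controller that sets up the multiplayer battle UI for the local player.
; On BeginPlay, only when the controller is local, it creates WBP_MultiBattleWidget and adds it to the viewport.
; It then shows the mouse cursor, switches player controller 0 to Game and UI input focused on that widget, enables input and prints a debug string.
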(event `self.ReceiveBeginPlay`
  (bind _returnvalue (`GameplayStatics.GetPlayerController` 0))
  (if (`self.IsLocalController`)
    (bind _returnvalue_2 (`|CreateWidget` "/Game/2_BP/Widget/WBP_MultiBattleWidget.WBP_MultiBattleWidget_C"))
    (`UserWidget.AddToViewport` _returnvalue_2 0)
    (set `PlayerController.bShowMouseCursor` true _returnvalue)
    (`WidgetBlueprintLibrary.SetInputMode_GameAndUIEx` _returnvalue _returnvalue_2)
    (`self.EnableInput` _returnvalue)
    (`KismetSystemLibrary.PrintString` "11")))

(fn `UserConstructionScript`)